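; Playable League of Legends-style Darius champion, implementing his auto attack, Hemorrhage passive and four spells.
; A per-target map, aged on Tick, tracks bleed stacks; a timer damages the latest target while BPCBlood animates stack marks.
; Five stacks grant Noxian Might's bonus AD.
; Spells are a two-zone healing spin, an AnimBP-swapping empowered attack, a timeline-driven cone pull and a stack-scaled ultimate limited to BP_Dummy targets.
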(event Custom|WCheck
  ;[0.15 0.02344 0.02344 0.5] Spell 2 Reset Auto
  (if (!= (Variables|Passif|GetAdditionalWDamage) 0.0)
    (Components|SkeletalMesh|SetAnimInstanceClass (Variables|Character|GetMesh) "/Game/LeagueOfLegends/Champion/Darius/Animations/ABP_Darius.ABP_Darius_C")
    (Variables|Default|SetIsCastingASpell? false)))

(event Custom|ApplyHemorrhage
  (params (Target :type Actor%20Object%20Reference))
  ;[0.5799 0.03492 0.7292 0.5] Passif System
  ;;[0.492 0.4353 0.7396 0.5] Apply the passif system
  (Variables|Passif|SetPassifTarget Target)
  (if (Utilities|Map|IsEmpty (Variables|Passif|GetBleedMap))
    (Variables|Passif|GetNoxianMight
      (:then
        (Variables|Passif|SetStacks 5))
      (:else
        (Variables|Passif|SetStacks 1)))
    (Utilities|Map|Add (Variables|Passif|GetBleedMap) (Variables|Passif|GetPassifTarget) (Utilities|Struct|MakeSBleedStruct (Variables|Passif|GetStacks) (Variables|Passif|GetBleedTime) (Variables|Passif|GetBleedDamage) 0.0))
    (else
      (bind _5stacks_ (CallFunction|Is5Stacks? (Variables|Passif|GetPassifTarget)))
      (if _5stacks_
        (CallFunction|MarkCheck)
        (bind _output_get (Variables|Passif|SetStacks 5))
        (Utilities|Map|Add (Variables|Passif|GetBleedMap) (Variables|Passif|GetPassifTarget) (Utilities|Struct|MakeSBleedStruct _output_get (Variables|Passif|GetBleedTime) (Variables|Passif|GetBleedDamage) 0.0))
        (else
          (bind _result (Math|Integer|IncrementInt (.stacks (.Value (Utilities|Map|Find (Variables|Passif|GetBleedMap) (Variables|Passif|GetPassifTarget)))))
            (:%20%20
              (Variables|Passif|SetStacks _result)
              (Utilities|Map|Add (Variables|Passif|GetBleedMap) (Variables|Passif|GetPassifTarget) (Utilities|Struct|MakeSBleedStruct _result (Variables|Passif|GetBleedTime) (Variables|Passif|GetBleedDamage) 0.0))))))))
  (Actor|Tick|SetActorTickEnabled true)
  ;;[1 0.2932 0.376 0.5] Apply the bleed damage
  (if (< (Variables|Passif|GetCurrentPlayerStack) (Variables|Passif|GetStacks))
    (Variables|Passif|SetCurrentPlayerStack (Variables|Passif|GetStacks)))
  (bind _returnvalue (Utilities|Time|SetTimerbyEvent (delegate Custom|ApplyBleedDamage) 1.2 true))
  (Variables|Passif|SetBleedTimer _returnvalue)
  (bind _output_get_2 (Variables|Passif|SetLastBloodIndex (.stacks (.Value (Utilities|Map|Find (Variables|Passif|GetBleedMap) (Variables|Passif|GetPassifTarget))))))
  (if (>= _output_get_2 2)
    (Default|DestroyLastMark (Variables|Default|GetBPC_Blood) (Variables|Passif|GetPassifTarget) (Variables|Passif|GetLastBloodIndex)))
  (Default|Apply (Variables|Default|GetBPC_Blood) (Variables|Passif|GetLastBloodIndex) (Variables|Passif|GetPassifTarget))
  (if (== (Variables|Passif|GetLastBloodIndex) 3)
    (Utilities|FlowControl|Sequence
      (:then_0
        (bind (_direction _cos _sin _cos2 _sin2) (Timeline|BloodAnimationTimeLine Stop)
          (:Update
            (Default|Animation (Variables|Default|GetBPC_Blood) (Variables|Passif|GetPassifTarget) _cos _cos2 _sin _sin2))
          (:Finished
            (Default|DestroyLastMark (Variables|Default|GetBPC_Blood) (Variables|Passif|GetPassifTarget) (Variables|Passif|GetLastBloodIndex)))))
      (:then_1
        (bind (_direction_2 _cos_2 _sin_2 _cos2_2 _sin2_2 _cos3 _sin3) (Timeline|BloodAnimation3Timeline PlayFromStart)
          (:Update
            (Default|Animfor3Stack (Variables|Default|GetBPC_Blood) (Variables|Passif|GetPassifTarget) _cos_2 _cos2_2 _cos3 _sin_2 _sin2_2 _sin3))
          (:Finished
            (Default|DestroyLastMark (Variables|Default|GetBPC_Blood) (Variables|Passif|GetPassifTarget) (Variables|Passif|GetLastBloodIndex))))))
    (else
      (Utilities|FlowControl|Sequence
        (:then_0
          (Timeline|BloodAnimation3Timeline Stop))
        (:then_1
          (Timeline|BloodAnimationTimeLine PlayFromStart))))))

(event Custom|CancleMark
  ;[0.5799 0.03492 0.7292 0.5] Passif System
  ;;[0.2783 0.113 1 0.5] Check and cancle Noxian Might
  (Variables|Passif|SetNoxianMight false)
  (Utilities|FlowControl|DelayUntilNextTick)
  (Variables|Passif|SetCurrentPlayerStack 0)
  (Variables|Passif|SetPassifAdditionalAD 0.0))

(event Custom|Rage
  ;[0.5799 0.03492 0.7292 0.5] Passif System
  ;;[1 0.2932 0.376 0.5] Apply the bleed damage
  (Default|Rage (Variables|Default|GetAs%20BP%20HUD%20LOL))
  (Audio|SpawnSound2D "/Game/LeagueOfLegends/Champion/Darius/Sound/P_Sound.P_Sound" 1.0 1.0 0.0 0))

(event Custom|ApplyBleedDamage
  (bind _passiftarget (Variables|Passif|GetPassifTarget))
  (bind _bleedmap (Variables|Passif|GetBleedMap))
  (bind _value (Utilities|Map|Find _bleedmap _passiftarget))
  ;[0.5799 0.03492 0.7292 0.5] Passif System
  ;;[1 0.2932 0.376 0.5] Apply the bleed damage
  (bind _output_get (Variables|Passif|SetEnemyStacks (.stacks _value)))
  (Game|Damage|ApplyDamage (Variables|Passif|GetPassifTarget) (* _output_get (.stacksdamage _value)) 0 0))

(event Custom|MarkCheck
  ;[0.5799 0.03492 0.7292 0.5] Passif System
  ;;[0.2783 0.113 1 0.5] Check and cancle Noxian Might
  (Variables|Passif|GetNoxianMight
    (:then
      (if (Class|KismetSystemLibrary|TimerExistsHandle (Variables|Passif|GetNoxianMightTimer))
        (Utilities|Time|ClearandInvalidateTimerbyHandle (Variables|Passif|GetNoxianMightTimer)))
      (bind _returnvalue (Utilities|Time|SetTimerbyEvent (delegate Custom|CancleMark) 5.0))
      (Variables|Passif|SetNoxianMightTimer _returnvalue))
    (:else)))

(event EventBeginPlay
  (|CallParentFunction)
  (Actor|Tick|SetActorTickEnabled false)
  (EventDispatchers|BindEventto5Stack (EventDispatchers|CreateEvent :!event Custom|Rage)))

(event EventTick
  (params (DeltaSeconds :type Float%20%28single-precision%29))
  (bind _bleedmap (Variables|Passif|GetBleedMap))
  ;[0.5799 0.03492 0.7292 0.5] Passif System
  ;;[0.3229 0.2489 0.6458 0.5] Manage the time of the passif
  (bind (_keypin _valuepin) (Utilities|Map|ForEachLoop(Map) _bleedmap)
    (:then
      (Utilities|Map|Add (Variables|Passif|GetBleedMap) _keypin (Utilities|Struct|MakeSBleedStruct (.stacks _valuepin) (- (.tempsrestants _valuepin) DeltaSeconds) (.stacksdamage _valuepin) (.dernierprock _valuepin)))
      (if (<= (.tempsrestants _valuepin) 0.0)
        (Utilities|FlowControl|DelayUntilNextTick)
        (Utilities|Map|Add (Variables|Passif|GetBleedMap) (Variables|Passif|GetPassifTarget) (Utilities|Struct|MakeSBleedStruct 0 (Variables|Passif|GetBleedTime) (Variables|Passif|GetBleedDamage) 0.0))
        (Utilities|Map|Remove (Variables|Passif|GetBleedMap) _keypin)
        (Utilities|Time|ClearandInvalidateTimerbyHandle (Variables|Passif|GetBleedTimer))))
    (:CompletedPin
      (if (Utilities|Map|IsEmpty _bleedmap)
        (Actor|Tick|SetActorTickEnabled false)))))

(event EventAttackCaC
  ;[0 0.5392 1 0.5] Auto Attack
  (bind _asbp_character (Utilities|Casting|CastToBP_Character (Variables|Default|GetHit%20Actor)))
  (Game|Damage|ApplyDamage _asbp_character (+ (Variables|Default|GetAttackDamage) (Variables|Passif|GetAdditionalWDamage) (Variables|Passif|GetPassifAdditionalAD)) 0 0 "/Script/Engine.DamageType")
  (CallFunction|ApplyHemorrhage _asbp_character)
  (if (!= (Variables|Passif|GetAdditionalWDamage) 0.0)
    (Audio|Components|Audio|Stop (Variables|Default|GetWSound))
    (Audio|SpawnSound2D "/Game/LeagueOfLegends/Champion/Darius/Sound/W_AA_Sound.W_AA_Sound" 1.0 1.0 0.0 0)
    (Variables|Passif|SetAdditionalWDamage 0.0)
    (Utilities|FlowControl|DelayUntilNextTick)
    (Components|SkeletalMesh|SetAnimInstanceClass (Variables|Character|GetMesh) "/Game/LeagueOfLegends/Champion/Darius/Animations/ABP_Darius.ABP_Darius_C")
    (Variables|Default|SetAnimation_AA_ToPlay (Variables|Animation|GetA%20AA%20Montage_0))
    (else
      (Audio|SpawnSound2D "/Game/LeagueOfLegends/Champion/Darius/Sound/AA_Sound.AA_Sound" 1.0 1.0 0.0 0))))

(event EventSpell1
  ;[0.03646 0.01304 0.01223 0.5] Spell 1 Spin
  (|CallParentFunction)
  (Audio|SpawnSound2D "/Game/LeagueOfLegends/Champion/Darius/Sound/Q_Sound.Q_Sound" 1.0 1.0 0.0 0)
  (Animation|Montage|PlayMontage (Variables|Character|GetMesh) "/Game/LeagueOfLegends/Champion/Darius/Animations/Montage_Animation/A_Spell1_Darius_Montage.A_Spell1_Darius_Montage"
    (:OnBlendOut
      (Animation|Montage|PlayMontage (Variables|Character|GetMesh) "/Game/LeagueOfLegends/Champion/Darius/Animations/Montage_Animation/A_Spell1_Spin_Darius_Montage.A_Spell1_Spin_Darius_Montage"
        (:then
          (bind (_outactors _returnvalue) (Collision|SphereOverlapActors (Transformation|GetActorLocation) (Variables|QSpell|GetQSharp) (Variables|Spell|GetObject%20Types) 0 (Utilities|Array|MakeArray self)))
          (if _returnvalue
            (for _array_element _outactors
              (if (< (Transformation|GetDistanceTo _array_element self) (Variables|QSpell|GetQBlunt))
                (Variables|QSpell|SetDamageQ (Variables|QSpell|GetBluntDamage))
                (else
                  (Variables|QSpell|SetDamageQ (Variables|QSpell|GetSharpDamage))
                  (CallFunction|ApplyHemorrhage _array_element)
                  (CallFunction|Heal (* (/ (- (Variables|Default|GetMaxHealth) (Variables|Default|GetHealth)) 1e+02) 17.0))))
              (Game|Damage|ApplyDamage _array_element (Variables|QSpell|GetDamageQ) 0 0))
            (Variables|Default|SetIsCastingASpell? false)
            (else
              (Development|PrintString "Pas de Cible Touché")
              (Variables|Default|SetIsCastingASpell? false))))))))

(event EventSpell2
  ;[0.15 0.02344 0.02344 0.5] Spell 2 Reset Auto
  (|CallParentFunction)
  (Components|SkeletalMesh|SetAnimInstanceClass (Variables|Character|GetMesh) "/Game/LeagueOfLegends/Champion/Darius/Animations/ABP_Darius_W.ABP_Darius_W_C")
  (Utilities|FlowControl|DelayUntilNextTick)
  (Utilities|Time|SetTimerbyEvent (delegate Custom|WCheck) 4.0)
  (Variables|Passif|SetAdditionalWDamage 4e+01)
  (Variables|Default|SetAnimation_AA_ToPlay (Variables|Animation|GetW%20AA%20Montage))
  (Variables|Default|SetIsCastingASpell? false)
  (bind _returnvalue (Audio|SpawnSound2D "/Game/LeagueOfLegends/Champion/Darius/Sound/W_Sound.W_Sound" 1.0 1.0 0.0 0))
  (Variables|Default|SetWSound _returnvalue))

(event EventSpell3
  (bind _actorhitbye (Variables|ESpell|GetActorHitByE))
  ;[0.6562 0.07519 0.07519 0.5] Spell 3 Grab
  (|CallParentFunction)
  (Audio|SpawnSound2D "/Game/LeagueOfLegends/Champion/Darius/Sound/E_Sound.E_Sound" 1.0 1.0 0.0 0)
  (Components|Movement|StopMovementImmediately (Variables|Character|GetCharacterMovement))
  (CallFunction|MakeFaceAPoint (.location (.HitResult (Game|Player|GetHitResultUnderCursorbyChannel (Game|GetPlayerController 0) "TraceTypeQuery1" true))))
  (Animation|Montage|PlayMontage (Variables|Character|GetMesh) "/Game/LeagueOfLegends/Champion/Darius/Animations/Montage_Animation/A_Spell3_Darius_Montage.A_Spell3_Darius_Montage"
    (:OnNotifyBegin
      (bind _outactors (Collision|SphereOverlapActors (Transformation|GetActorLocation) (Variables|ESpell|GetERange) (Variables|Spell|GetObject%20Types) 0 (Utilities|Array|MakeArray self)))
      (for _array_element _outactors
        (Variables|ESpell|SetArray%20Element _array_element)
        (if (>= (Class|KismetMathLibrary|DegAcos (Math|Vector|DotProduct (Transformation|GetActorForwardVector self) (Math|Vector|Normalize (- (Transformation|GetActorLocation) (Transformation|GetActorLocation _array_element))))) 1.5e+02)
          (Utilities|Array|AddUnique (Variables|ESpell|GetActorHitByE) (Variables|ESpell|GetArray%20Element))
          (else
            (Development|PrintString "No Hit"))))
      (if (Utilities|Array|IsNotEmpty _actorhitbye)
        (Utilities|Array|Clear (Variables|ESpell|GetStartGrab))
        (for _array_element_2 _actorhitbye
          (Utilities|Array|Add (Variables|ESpell|GetStartGrab) (Transformation|GetActorLocation _array_element_2)))
        (Variables|ESpell|SetEndGrab (Transformation|GetActorLocation))
        (bind _newtrack_0 (Timeline|GrabTimelien PlayFromStart)
          (:Update
            (for (_array_element_3 _array_index) (Variables|ESpell|GetActorHitByE)
              (Transformation|SetActorLocation _array_element_3 (Math|Vector|Lerp(Vector) (Utilities|Array|Get(acopy) (Variables|ESpell|GetStartGrab) _array_index) (Variables|ESpell|GetEndGrab) _newtrack_0) true false)))
          (:Finished
            (Utilities|FlowControl|DelayUntilNextTick)
            (Utilities|Array|Clear (Variables|ESpell|GetActorHitByE))
            (Variables|Default|SetIsCastingASpell? false)))
        (else
          (Variables|Default|SetIsCastingASpell? false))))))

(event EventSpell4
  ;[1 0.01064 0 0.5] Ultimate
  (bind _output_get (Variables|Ultimate|SetEnemyInRangeOfUltimate (.hitactor (.HitResult (Game|Player|GetHitResultUnderCursorbyChannel (Game|GetPlayerController 0) "TraceTypeQuery1" true)))))
  (bind _is_in_range_ (CallFunction|RangeCheck (Transformation|GetActorLocation) (Transformation|GetActorLocation _output_get) (Variables|Ultimate|GetRangeUltimate)))
  (Class|KismetSystemLibrary|IsObjectOfSoftClass (Variables|Ultimate|GetEnemyInRangeOfUltimate) "/Game/LeagueOfLegends/Champion/Dummy/BP_Dummy.BP_Dummy_C"
    (:True
      (if _is_in_range_
        (Audio|SpawnSound2D "/Game/LeagueOfLegends/Champion/Darius/Sound/R_Sound.R_Sound" 1.0 1.0 0.0 0)
        (Pawn|Components|CharacterMovement|DisableMovement (Variables|Character|GetCharacterMovement))
        (|CallParentFunction)
        (CallFunction|MakeFaceAPoint (Transformation|GetActorLocation (Variables|Ultimate|GetEnemyInRangeOfUltimate)))
        (Animation|Montage|PlayMontage (Variables|Character|GetMesh) "/Game/LeagueOfLegends/Champion/Darius/Animations/Montage_Animation/A_Spell4_Darius_Montage.A_Spell4_Darius_Montage"
          (:OnCompleted
            (Variables|Default|SetIsCastingASpell? false))
          (:OnNotifyBegin
            (Game|Damage|ApplyDamage (Variables|Ultimate|GetEnemyInRangeOfUltimate) (* (Variables|Ultimate|GetUltimateDamage) (Utilities|Array|Get(acopy) (Variables|Passif|GetPassifR%25Damage) (Variables|Passif|GetCurrentPlayerStack))) 0 0)
            (Pawn|Components|CharacterMovement|SetMovementMode (Variables|Character|GetCharacterMovement) "MOVE_Walking" 0)
            (CallFunction|ApplyHemorrhage (Variables|Ultimate|GetEnemyInRangeOfUltimate))))
        (else
          (Utilities|FlowControl|DelayUntilNextTick :!label _label)
          (Variables|Default|SetIsCastingASpell? false)
          (Development|PrintString "caca"))))
    (:False
      (goto _label))))

(fn ConstructionScript
  (|CallParentFunction))

(fn Is5Stacks?
  (params (ActorToCheck :type Actor%20Object%20Reference%20%28by%20ref%29))
  (if (>= (.stacks (.Value (Utilities|Map|Find (Variables|Passif|GetBleedMap) ActorToCheck))) 4)
    (bind _output_get (Variables|Passif|SetNoxianMight true))
    (Default|Call5Stack)
    (Variables|Passif|SetPassifAdditionalAD 3e+01)
    (return _output_get)
    (else
      (bind _output_get_2 (Variables|Passif|SetNoxianMight false))
      (Variables|Passif|SetPassifAdditionalAD 0.0)
      (return _output_get_2))))