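; BP_Dummy is a target dummy champion that shows the damage it takes and restores itself to full health afterward.
; Each hit runs the parent damage logic, displays the amount in colored world text, and restarts a retriggerable delay.
; When that delay expires without further hits, it resets Health to MaxHealth, updates the health bar widget and shows heal text.
; The shared TextUpdate event clears the text after a short delay.
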(event Custom|TextUpdate
  (params (Value :type Text%20%28by%20ref%29) (Value2 :type Color%20Structure))
  ;[0.06301 0.1095 0.05781] 5 Secondes after taking Damage, he heal Full life automaticly
  (Rendering|Components|TextRender|SetText (Variables|Default|GetDAMAGE) Value)
  (Rendering|Components|TextRender|SetTextRenderColor (Variables|Default|GetDAMAGE) Value2)
  (Utilities|FlowControl|Delay 1.0)
  (Rendering|Components|TextRender|SetText (Variables|Default|GetDAMAGE) (Class|KismetTextLibrary|GetEmptyText)))

(event EventBeginPlay
  ;[0.06301 0.1095 0.05781] 5 Secondes after taking Damage, he heal Full life automaticly
  (|CallParentFunction))

(event Game|Damage|EventAnyDamage
  (params (Damage :type Float%20%28single-precision%29) (DamageType :type Damage%20Type%20Object%20Reference) (InstigatedBy :type Controller%20Object%20Reference) (DamageCauser :type Actor%20Object%20Reference))
  (bind _maxhealth (Variables|Default|GetMaxHealth))
  ;[0.06301 0.1095 0.05781] 5 Secondes after taking Damage, he heal Full life automaticly
  (|CallParentFunction Damage DamageType InstigatedBy DamageCauser)
  (CallFunction|TextUpdate (Utilities|Text|ToText(Float) Damage "HalfToEven") (Variables|Default|GetColor%20Damage))
  (Utilities|FlowControl|RetriggerableDelay (Variables|Default|GetResetTimer))
  (bind _output_get (Variables|Default|SetHealth _maxhealth))
  (Default|HealthBarUpdate (Variables|Default|GetAs%20WBP%20Health%20Bar) (/ _output_get _maxhealth))
  (CallFunction|TextUpdate (Variables|Default|GetTextHeal) (Variables|Default|GetColorHeal)))

(fn ConstructionScript
  (|CallParentFunction))