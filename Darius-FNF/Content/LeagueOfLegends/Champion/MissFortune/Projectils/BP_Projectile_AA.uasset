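; Miss Fortune auto-attack projectile that homes through its ProjectileMovement component and expires after a fixed delay.
; On spawn it caches the player character's HitActor and assigns its homing target component.
; Tick copies the character's enemy location into TargetLocation, which nothing in the graph reads.
; Sphere overlap with HitActor destroys the projectile, with damage only a debug print.
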(event OnComponentBeginOverlap(Sphere1)
  (params (OverlappedComponent :type Primitive%20Component%20Object%20Reference) (OtherActor :type Actor%20Object%20Reference) (OtherComp :type Primitive%20Component%20Object%20Reference) (OtherBodyIndex :type Integer) (bFromSweep :type Boolean) (SweepResult :type Hit%20Result%20Structure%20%28by%20ref%29))
  (Development|PrintString "Hello")
  (if (== OtherActor (Variables|Default|GetHit%20Actor))
    (Actor|DestroyActor)
    (Development|PrintString "Damage")))

(event EventBeginPlay
  (bind _asbp_character (Utilities|Casting|CastToBP_Character (Game|GetPlayerCharacter 0)))
  (bind _output_get (Variables|Default|SetAs%20BP%20Character _asbp_character))
  (Variables|/Script/Engine.ProjectileMovementComponent|SetHomingTargetComponent (Variables|Default|GetProjectileMovement) (Variables|Default|GetHoming%20Target%20Component))
  (Variables|Default|SetHit%20Actor (Variables|/Game/LeagueOfLegends/Character/BP_Character.BP_Character_C|GetHit%20Actor _output_get))
  (Utilities|FlowControl|Delay 5.0)
  (Actor|DestroyActor))

(event Collision|EventActorBeginOverlap
  (params (OtherActor :type Actor%20Object%20Reference)))

(event EventTick
  (params (DeltaSeconds :type Float%20%28single-precision%29))
  (Variables|Default|SetTargetLocation (Math|Conversions|ToTransform(Vector) (Variables|/Game/LeagueOfLegends/Character/BP_Character.BP_Character_C|GetEnemiLocation (Variables|Default|GetAs%20BP%20Character)))))

(fn ConstructionScript)