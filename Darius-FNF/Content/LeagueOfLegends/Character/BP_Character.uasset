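; League of Legends-style player character with click-to-move, auto-attacks, four spells, health and mana.
; Right-click traces under the cursor, then moves there or attacks a BP_Dummy, approaching first if out of range.
; Spell inputs check mana, cooldown and active casting, then call per-spell events that spend mana and start Delay-based cooldowns.
; Damage, healing and regen update the HUD and overhead bar; extras include range indicators, pause and a no-cost toggle.
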(event Custom|Fire
  (bind _mesh (Variables|Character|GetMesh))
  ;[0.15 0.15 0.15 0.5] System To attack as a Mele Range or Long Range
  (bind _returnvalue (AddComponent|AddSceneComponent (Variables|AA|GetHit%20Actor) false))
  (Game|SpawnActorfromClass "/Game/LeagueOfLegends/Champion/MissFortune/Projectils/BP_Projectile_AA.BP_Projectile_AA_C" (Math|Transform|MakeTransform (Transformation|GetSocketLocation _mesh (Variables|AA|GetSocket%20Porjectil)) (Math|Rotator|MakeRotator 0.0 0.0 (+ 9e+01 (.yaw (Transformation|GetWorldRotation _mesh)))) "1.000000,1.000000,1.000000") "Undefined" "MultiplyWithRoot" 0 _returnvalue 0))

(event Custom|AA
  ;[0.15 0.15 0.15 0.5] ClassicAutoAttack
  (Variables|CoolDown|SetCanAA? false)
  (CallFunction|MakeFaceAPoint (Variables|AA|GetEnemiLocation))
  (Animation|Montage|PlayMontage (Variables|Character|GetMesh) (Variables|Animation|GetAnimation_AA_ToPlay) 1.0 0.0 "None" false
    (:OnCompleted
      _)
    (:OnInterrupted
      _))
  (Variables|CoolDown|SetCanAA? true))

(event Custom|AutoRegen
  ;[0.03955 0.6654 0] Restor Mana and Health Automaticly
  (if (== (Game|Player|GetPlayerPawn 0) self)
    (Utilities|FlowControl|Sequence
      (:then_0
        (if (!= (Variables|Mana|GetManaMax) (Variables|Mana|GetManaCurrent))
          (bind _output_get (Variables|Mana|SetManaCurrent (Math|Float|Clamp(Float) (+ (Variables|Mana|GetManaCurrent) (Variables|Mana|GetManaRegenPs)) 0.0 (Variables|Mana|GetManaMax))))
          (Default|ManaBarUpdate (Variables|HUD|GetAs%20WBP%20Health%20Bar) (/ _output_get (Variables|Mana|GetManaMax)))
          (Default|UpdateMana (Variables|HUD|GetAs%20BP%20HUD%20LOL) (/ _output_get (Variables|Mana|GetManaMax)) _output_get)))
      (:then_1
        (if (!= (Variables|Health|GetMaxHealth) (Variables|Health|GetHealth))
          (bind _output_get_2 (Variables|Health|SetHealth (Math|Float|Clamp(Float) (+ (Variables|Health|GetHealth) (Variables|Health|GetHealPs)) 0.0 (Variables|Health|GetMaxHealth))))
          (Default|HealthBarUpdate (Variables|HUD|GetAs%20WBP%20Health%20Bar) (/ _output_get_2 (Variables|Health|GetMaxHealth)))
          (Default|UpdateLife (Variables|HUD|GetAs%20BP%20HUD%20LOL) (/ _output_get_2 (Variables|Health|GetMaxHealth)) _output_get_2))))))

(event Custom|UseMana
  (params (ManaCost :type Float%20%28double-precision%29))
  ;[0.06687 0.7552 0.7544 0.5] Spells System
  (bind _output_get (Variables|Mana|SetManaCurrent (- (Variables|Mana|GetManaCurrent) ManaCost)))
  (Default|ManaBarUpdate (Variables|HUD|GetAs%20WBP%20Health%20Bar) (/ _output_get (Variables|Mana|GetManaMax)))
  (Default|UpdateMana (Variables|HUD|GetAs%20BP%20HUD%20LOL) (/ _output_get (Variables|Mana|GetManaMax)) _output_get)
  (Audio|SpawnSound2D "/Game/LeagueOfLegends/Sound/Spell.Spell" 1.0 1.0 0.0 0))

(event Custom|SetRangeOfSpellVisible
  (params (Range :type Static%20Mesh%20Component%20Object%20Reference) (InputPin :type Float%20%28double-precision%29))
  ;[0.06687 0.7552 0.7544 0.5] Spells System
  (if (and (> InputPin (Variables|Spells|GetVisibilityRangeWaitingTime)) (not (Variables|Spells|GetIsCastingASpell?)))
    (Rendering|SetVisibility Range true false)))

(event Custom|Can'tCast
  (params (NotEneathMana? :type Boolean))
  ;[0.06687 0.7552 0.7544 0.5] Spells System
  (Audio|SpawnSound2D (select NotEneathMana? "/Game/LeagueOfLegends/Sound/InCouldown.InCouldown" "/Game/LeagueOfLegends/Sound/Mana.Mana") 1.0 1.0 0.0 0))

(event Custom|Die
  ;[0.07819 0.1912 0.3005] BeginPlay
  (Default|CallOnCharacterDie))

(event Custom|CancleAnimation
  (bind _animation_aa_toplay (Variables|Animation|GetAnimation_AA_ToPlay))
  ;[0.15 0.15 0.15 0.5] Cancle the animation like in the game when you spam S to cancle the animation of the character
  (Utilities|IsValid _animation_aa_toplay
    (:Is%20Valid
      (Animation|StopAnimMontage _animation_aa_toplay))))

(event Custom|CastSpell
  (params (index :type Integer) (ManaCost :type Float%20%28double-precision%29))
  ;[0.06687 0.7552 0.7544 0.5] Spells System
  (CallFunction|CooldownSet index)
  (CallFunction|UseMana ManaCost))

(event Custom|CooldownSet
  (params (index :type Integer))
  ;[0 0.15 0.01088 0.5] Couldown
  (switch int index
    (:0
      (Variables|CoolDown|SetCooldownQ (Variables|CoolDown|GetInisial_CooldownQ)))
    (:1
      (Variables|CoolDown|SetCooldownW (Variables|CoolDown|GetInisial_CooldownW)))
    (:2
      (Variables|CoolDown|SetCooldownE (Variables|CoolDown|GetInisial_CooldownE)))
    (:3
      (Variables|CoolDown|SetCooldownR (Variables|CoolDown|GetInisial_CooldownR))))
  (Default|CooldownSystem (Variables|HUD|GetAs%20BP%20HUD%20LOL) index)
  (switch int index
    (:0
      (CallFunction|CoolDownforQ))
    (:1
      (CallFunction|CoolDownforW))
    (:2
      (CallFunction|CoolDownforE))
    (:3
      (CallFunction|CoolDownforR))))

(event Custom|AttackCaC
  ;[0.15 0.15 0.15 0.5] System To attack as a Mele Range or Long Range
  (Development|PrintString "CAC"))

(event Custom|CoolDownForR
  ;[0 0.15 0.01088 0.5] Couldown
  (Utilities|FlowControl|Delay (Variables|CoolDown|GetInisial_CooldownR))
  (Variables|CoolDown|SetCooldownR 0.0)
  (Variables|CoolDown|SetResetIndex 3)
  (Default|Reset (Variables|HUD|GetAs%20BP%20HUD%20LOL) (Variables|CoolDown|GetResetIndex)))

(event Custom|CoolDownForQ
  ;[0 0.15 0.01088 0.5] Couldown
  (Utilities|FlowControl|Delay (Variables|CoolDown|GetInisial_CooldownQ))
  (Variables|CoolDown|SetCooldownQ 0.0)
  (Variables|CoolDown|SetResetIndex 0)
  (Default|Reset (Variables|HUD|GetAs%20BP%20HUD%20LOL) (Variables|CoolDown|GetResetIndex)))

(event Custom|CoolDownForW
  ;[0 0.15 0.01088 0.5] Couldown
  (Utilities|FlowControl|Delay (Variables|CoolDown|GetInisial_CooldownW))
  (Variables|CoolDown|SetCooldownW 0.0)
  (Variables|CoolDown|SetResetIndex 1)
  (Default|Reset (Variables|HUD|GetAs%20BP%20HUD%20LOL) (Variables|CoolDown|GetResetIndex)))

(event Custom|CoolDownForE
  ;[0 0.15 0.01088 0.5] Couldown
  (Utilities|FlowControl|Delay (Variables|CoolDown|GetInisial_CooldownE))
  (Variables|CoolDown|SetCooldownE 0.0)
  (Variables|CoolDown|SetResetIndex 2)
  (Default|Reset (Variables|HUD|GetAs%20BP%20HUD%20LOL) (Variables|CoolDown|GetResetIndex)))

(event Custom|Heal
  (params (Amount :type Float%20%28double-precision%29))
  ;[0.01711 0.15 0 0.5] Heal For Spell
  (bind _output_get (Variables|Health|SetHealth (Math|Float|Clamp(Float) (+ (Variables|Health|GetHealth) Amount) (Variables|Health|GetHealth) (Variables|Health|GetMaxHealth))))
  (Default|UpdateLife (Variables|HUD|GetAs%20BP%20HUD%20LOL) (/ _output_get (Variables|Health|GetMaxHealth)) _output_get)
  (Default|HealthBarUpdate (Variables|HUD|GetAs%20WBP%20Health%20Bar) (/ _output_get (Variables|Health|GetMaxHealth))))

(event Custom|Spell4
  ;[0.06687 0.7552 0.7544 0.5] Spells System
  (CallFunction|CastSpell 3 (Variables|Mana|GetSpell%204%20Cost)))

(event Custom|Spell1
  ;[0.06687 0.7552 0.7544 0.5] Spells System
  (CallFunction|CastSpell 0 (Variables|Mana|GetSpell%201%20Cost)))

(event Custom|Make%20Face%20A%20Point
  (params (Target :type Vector))
  ;[0.000607 0.3095 0.6867] Make an actor Look where something is
  (Transformation|SetWorldRotation (Variables|Collision|GetCapsuleComponent) (Math|Rotator|MakeRotator 0.0 0.0 (- (.Yaw (Math|Rotator|BreakRotator (Math|Rotator|FindLookatRotation (Transformation|GetActorLocation) Target))) (.yaw (Pawn|GetControlRotation :!class /Script/Engine.Pawn)))) false false))

(event Custom|Spell2
  ;[0.06687 0.7552 0.7544 0.5] Spells System
  (CallFunction|CastSpell 1 (Variables|Mana|GetSpell%202%20Cost)))

(event Custom|NoCostSystem
  ;[0.15 0.0471 0 0.5] No Cost Mode
  (Utilities|FlowControl|FlipFlop
    (:A
      (bind _output_get (Variables|CoolDown|SetInisial_CooldownQ (Math|Float|MakeLiteralFloat 0.0)))
      (bind _output_get_2 (Variables|CoolDown|SetInisial_CooldownW _output_get))
      (bind _output_get_3 (Variables|CoolDown|SetInisial_CooldownE _output_get_2))
      (bind _output_get_4 (Variables|CoolDown|SetInisial_CooldownR _output_get_3))
      (bind _output_get_5 (Variables|Mana|SetSpell%201%20Cost _output_get_4))
      (bind _output_get_6 (Variables|Mana|SetSpell%202%20Cost _output_get_5))
      (bind _output_get_7 (Variables|Mana|SetSpell%203%20Cost _output_get_6))
      (Variables|Mana|SetSpell%204%20Cost _output_get_7))
    (:B
      (Variables|CoolDown|SetInisial_CooldownQ (Utilities|Array|Get(acopy) (Variables|CoolDown|GetInisial_CooldownArray) (Variables|CoolDown|GetIndexNOCOST)))
      (Math|Integer|IncrementInt (Variables|CoolDown|GetIndexNOCOST)
        (:%20%20
          (Variables|CoolDown|SetInisial_CooldownW (Utilities|Array|Get(acopy) (Variables|CoolDown|GetInisial_CooldownArray) (Variables|CoolDown|GetIndexNOCOST)))
          (Math|Integer|IncrementInt (Variables|CoolDown|GetIndexNOCOST)
            (:%20%20
              (Variables|CoolDown|SetInisial_CooldownE (Utilities|Array|Get(acopy) (Variables|CoolDown|GetInisial_CooldownArray) (Variables|CoolDown|GetIndexNOCOST)))
              (Math|Integer|IncrementInt (Variables|CoolDown|GetIndexNOCOST)
                (:%20%20
                  (Variables|CoolDown|SetInisial_CooldownR (Utilities|Array|Get(acopy) (Variables|CoolDown|GetInisial_CooldownArray) (Variables|CoolDown|GetIndexNOCOST)))
                  (Variables|CoolDown|SetIndexNOCOST 0)
                  (Variables|Mana|SetSpell%201%20Cost (Utilities|Array|Get(acopy) (Variables|Mana|GetInisial_Mana_Cost) (Variables|CoolDown|GetIndexNOCOST)))
                  (Math|Integer|IncrementInt (Variables|CoolDown|GetIndexNOCOST)
                    (:%20%20
                      (Variables|Mana|SetSpell%202%20Cost (Utilities|Array|Get(acopy) (Variables|Mana|GetInisial_Mana_Cost) (Variables|CoolDown|GetIndexNOCOST)))
                      (Math|Integer|IncrementInt (Variables|CoolDown|GetIndexNOCOST)
                        (:%20%20
                          (Variables|Mana|SetSpell%203%20Cost (Utilities|Array|Get(acopy) (Variables|Mana|GetInisial_Mana_Cost) (Variables|CoolDown|GetIndexNOCOST)))
                          (Math|Integer|IncrementInt (Variables|CoolDown|GetIndexNOCOST)
                            (:%20%20
                              (Variables|Mana|SetSpell%204%20Cost (Utilities|Array|Get(acopy) (Variables|Mana|GetInisial_Mana_Cost) (Variables|CoolDown|GetIndexNOCOST)))
                              (Variables|CoolDown|SetIndexNOCOST 0))))))))))))))))

(event Custom|Spell3
  ;[0.06687 0.7552 0.7544 0.5] Spells System
  (CallFunction|CastSpell 2 (Variables|Mana|GetSpell%203%20Cost)))

(event Input|EnhancedActionEvents|EnhancedInputActionIA_RightClick
  (params (ActionValue :type Boolean) (ElapsedSeconds :type Float%20%28double-precision%29) (TriggeredSeconds :type Float%20%28double-precision%29) (InputAction :type Input%20Action%20Object%20Reference :default "/Game/LeagueOfLegends/Input/IA_RightClick.IA_RightClick"))
  (bind _returnvalue (Game|GetPlayerController 0))
  (bind (_worldlocation _worlddirection) (Game|Player|ConvertMouseLocationToWorldSpace _returnvalue))
  ;[1 1 1] Movement
  ;;[0 1 0 0.5] When i right click
  (:Started
    ;;;[0 0.06395 0.5938 0.5] Creat a LineTrace from the camera to the Cursor position
    (Utilities|IsValid (Variables|Animation|GetAnimeIdleIn)
      (:Is%20Valid
        (Animation|Montage|MontageStop (Components|SkeletalMesh|GetAnimInstance (Variables|Character|GetMesh)) 0.0 (Variables|Animation|GetAnimeIdleIn)))
      (:Is%20Not%20Valid
        _))
    (bind (_outhit _returnvalue_2) (Collision|LineTraceByChannel _worldlocation (+ _worldlocation (* _worlddirection (Math|Float|MakeLiteralFloat 1e+07))) "TraceTypeQuery1" true 0 "ForDuration"))
    (if _returnvalue_2
      ;;;[0.9823 0.5776 0.01681] Set All the Variable for later
      (Variables|AA|SetHit%20Actor (.HitActor (Collision|BreakHitResult _outhit)))
      (Variables|AA|SetLocation (.Location (Collision|BreakHitResult _outhit)))
      (Variables|AA|SetEnemiLocation (Transformation|GetActorLocation (Variables|AA|GetHit%20Actor)))
      (Variables|AA|SetPosition (Transformation|GetActorLocation (Game|GetPlayerCharacter 0)))
      ;;;[0.1559 0.117 0.0356] Check is the other actor is in range
      (if (== "/Game/LeagueOfLegends/Champion/Dummy/BP_Dummy.BP_Dummy_C" (Utilities|GetClass (Variables|AA|GetHit%20Actor)))
        (bind _is_in_range_ (CallFunction|RangeCheck (Variables|AA|GetPosition) (Variables|AA|GetEnemiLocation) (Variables|AA|GetRange)))
        (if (and _is_in_range_ (Variables|CoolDown|GetCanAA?))
          (Components|Movement|StopMovementImmediately (Variables|Character|GetCharacterMovement))
          (if true
            (CallFunction|AA))
          (else
            (bind _positionforattack (CallFunction|PostionforAttack (Variables|AA|GetRange)))
            (AI|Navigation|SimpleMovetoLocation (Game|GetPlayerController 0) _positionforattack)))
        (else
          (AI|Navigation|SimpleMovetoLocation (Game|GetPlayerController 0) (Variables|AA|GetLocation))
          (CallFunction|CancleAnimation)
          (Variables|CoolDown|SetCanAA? true))))))

(event Input|EnhancedActionEvents|EnhancedInputActionAI_StopMoving
  (params (ActionValue :type Boolean) (ElapsedSeconds :type Float%20%28double-precision%29) (TriggeredSeconds :type Float%20%28double-precision%29) (InputAction :type Input%20Action%20Object%20Reference :default "/Game/LeagueOfLegends/Input/AI_StopMoving.AI_StopMoving"))
  (bind _mesh (Variables|Character|GetMesh))
  (bind _returnvalue (Components|SkeletalMesh|GetAnimInstance _mesh))
  ;[1 1 1] Movement
  ;;[0 0.3338 0.7448 0.5] Stop Movement By Pressing S
  (Components|Movement|StopMovementImmediately (Variables|Character|GetCharacterMovement))
  (Utilities|IsValid _returnvalue
    (:Is%20Valid
      (Animation|Montage|MontageStop _returnvalue 0.0 "/Game/LeagueOfLegends/Champion/MissFortune/Animations/Montage_Animation/A_AA_Montage.A_AA_Montage"))
    (:Is%20Not%20Valid
      _))
  (if (Variables|Animation|GetIdleIn?)
    (Animation|PlayAnimMontage (Variables|Animation|GetAnimeIdleIn) 1.0 "None")))

(event Input|EnhancedActionEvents|EnhancedInputActionAI_Spell1
  (params (ActionValue :type Boolean) (ElapsedSeconds :type Float%20%28double-precision%29) (TriggeredSeconds :type Float%20%28double-precision%29) (InputAction :type Input%20Action%20Object%20Reference :default "/Game/LeagueOfLegends/Input/AI_Spell1.AI_Spell1"))
  (bind _spell1range (Variables|Default|GetSpell1Range))
  ;[0.06687 0.7552 0.7544 0.5] Spells System
  (:Triggered
    (bind (_cancast_ _mana_) (CallFunction|CanCasttheSpell? (Variables|Mana|GetSpell%201%20Cost) (Variables|CoolDown|GetCooldownQ) _spell1range))
    (if _cancast_
      (CallFunction|Spell1)
      (Variables|Spells|SetIsCastingASpell? true)
      (else
        (CallFunction|Can'tCast _mana_))))
  (:Ongoing
    (CallFunction|SetRangeOfSpellVisible _spell1range ElapsedSeconds)))

(event Input|EnhancedActionEvents|EnhancedInputActionAI_Spell2
  (params (ActionValue :type Boolean) (ElapsedSeconds :type Float%20%28double-precision%29) (TriggeredSeconds :type Float%20%28double-precision%29) (InputAction :type Input%20Action%20Object%20Reference :default "/Game/LeagueOfLegends/Input/AI_Spell2.AI_Spell2"))
  (bind _spell2range (Variables|Default|GetSpell2Range))
  ;[0.06687 0.7552 0.7544 0.5] Spells System
  (:Triggered
    (bind (_cancast_ _mana_) (CallFunction|CanCasttheSpell? (Variables|Mana|GetSpell%202%20Cost) (Variables|CoolDown|GetCooldownW) _spell2range))
    (if _cancast_
      (CallFunction|Spell2)
      (Variables|Spells|SetIsCastingASpell? true)
      (else
        (CallFunction|Can'tCast _mana_))))
  (:Ongoing
    (CallFunction|SetRangeOfSpellVisible _spell2range ElapsedSeconds)))

(event Input|EnhancedActionEvents|EnhancedInputActionAI_Spell3
  (params (ActionValue :type Boolean) (ElapsedSeconds :type Float%20%28double-precision%29) (TriggeredSeconds :type Float%20%28double-precision%29) (InputAction :type Input%20Action%20Object%20Reference :default "/Game/LeagueOfLegends/Input/AI_Spell3.AI_Spell3"))
  (bind _spell3range (Variables|Default|GetSpell3range))
  ;[0.06687 0.7552 0.7544 0.5] Spells System
  (:Triggered
    (bind (_cancast_ _mana_) (CallFunction|CanCasttheSpell? (Variables|Mana|GetSpell%203%20Cost) (Variables|CoolDown|GetCooldownE) _spell3range))
    (if _cancast_
      (CallFunction|Spell3)
      (Variables|Spells|SetIsCastingASpell? true)
      (else
        (CallFunction|Can'tCast _mana_))))
  (:Ongoing
    (CallFunction|SetRangeOfSpellVisible _spell3range ElapsedSeconds)))

(event Input|EnhancedActionEvents|EnhancedInputActionAI_Spell4
  (params (ActionValue :type Boolean) (ElapsedSeconds :type Float%20%28double-precision%29) (TriggeredSeconds :type Float%20%28double-precision%29) (InputAction :type Input%20Action%20Object%20Reference :default "/Game/LeagueOfLegends/Input/AI_Spell4.AI_Spell4"))
  (bind _spell4range (Variables|Default|GetSpell4range))
  ;[0.06687 0.7552 0.7544 0.5] Spells System
  (:Triggered
    (bind (_cancast_ _mana_) (CallFunction|CanCasttheSpell? (Variables|Mana|GetSpell%204%20Cost) (Variables|CoolDown|GetCooldownR) _spell4range))
    (if _cancast_
      (CallFunction|Spell4)
      (Variables|Spells|SetIsCastingASpell? true)
      (else
        (CallFunction|Can'tCast _mana_))))
  (:Ongoing
    (CallFunction|SetRangeOfSpellVisible _spell4range ElapsedSeconds)))

(event Input|EnhancedActionEvents|EnhancedInputActionAI_Stat
  (params (ActionValue :type Boolean) (ElapsedSeconds :type Float%20%28double-precision%29) (TriggeredSeconds :type Float%20%28double-precision%29) (InputAction :type Input%20Action%20Object%20Reference :default "/Game/LeagueOfLegends/Input/AI_Stat.AI_Stat"))
  (bind _rangecircle (Variables|Default|GetRangeCircle))
  ;[0.7755 0.5625 1] Make the Range Visible
  (:Triggered
    (Rendering|SetVisibility _rangecircle true false))
  (:Canceled
    (Rendering|SetVisibility _rangecircle false false :!label _label))
  (:Completed
    (goto _label)))

(event Input|EnhancedActionEvents|EnhancedInputActionAI_Pause
  (params (ActionValue :type Boolean) (ElapsedSeconds :type Float%20%28double-precision%29) (TriggeredSeconds :type Float%20%28double-precision%29) (InputAction :type Input%20Action%20Object%20Reference :default "/Game/LeagueOfLegends/Input/AI_Pause.AI_Pause"))
  (bind _returnvalue (Game|GetPlayerController 0))
  ;[0.05286 0.001518 0.2346] Pause the game
  (Game|SetGamePaused true)
  (bind _returnvalue_2 (UserInterface|CreateWidget "/Game/LeagueOfLegends/Widgets/WBP_Pause.WBP_Pause_C" 0 0))
  (bind _output_get (Variables|Menu|SetWBP_Pause _returnvalue_2))
  (Variables|/Game/LeagueOfLegends/Widgets/WBP_Pause.WBP_Pause_C|SetBP_Player _output_get self)
  (UserInterface|Viewport|AddtoViewport _output_get 0)
  (Input|SetInputModeGameandUI _returnvalue _output_get "DoNotLock" true false)
  (Variables|/Script/Engine.PlayerController|SetbShowMouseCursor _returnvalue true))

(event EventBeginPlay
  (bind _returnvalue (Game|GetPlayerController 0))
  (bind _range (Variables|AA|GetRange))
  (bind _rangecircle (Variables|Default|GetRangeCircle))
  (bind _returnvalue_2 (Transformation|GetWorldScale _rangecircle))
  (bind _returnvalue_3 (/ _range 5e+01))
  ;[0.07819 0.1912 0.3005] BeginPlay
  ;;[0.855 0.9734 0.3916] Mapping + cursor
  (Input|AddMappingContext (PlayerController|LocalPlayerSubsystems|GetEnhancedInputLocalPlayerSubsystem _returnvalue) "/Game/LeagueOfLegends/Input/IMC.IMC" 0 "(bIgnoreAllPressedKeysUntilRelease=True,bForceImmediately=False,bNotifyUserSettings=False)")
  (Variables|/Script/Engine.PlayerController|SetbShowMouseCursor _returnvalue true)
  (bind _asbp_hud_lol (Utilities|Casting|CastToBP_HUD_LOL (HUD|GetHUD (Game|GetPlayerController 0))))
  (Variables|HUD|SetAs%20BP%20HUD%20LOL _asbp_hud_lol)
  ;;[0 0.3968 0.9047] Set The Size of the Cercle Under the Player with the Range
  (Transformation|SetRelativeScale3D (Variables|Default|GetRangeCircle) (Math|Vector|MakeVector (* _returnvalue_3 (.x _returnvalue_2)) (* _returnvalue_3 (.y _returnvalue_2)) (.z _returnvalue_2)))
  ;;[0.03955 0.6445 0] Set Start Stat
  (Variables|Mana|SetManaCurrent (Variables|Mana|GetManaMax))
  (Variables|Health|SetHealth (Variables|Health|GetMaxHealth))
  (bind _aswbp_health_bar (Utilities|Casting|CastToWBP_HealthBar (UserInterface|GetWidget (Variables|Default|GetWidget))))
  (Variables|HUD|SetAs%20WBP%20Health%20Bar _aswbp_health_bar)
  (Variables|CoolDown|SetInisial_CooldownArray (Utilities|Array|MakeArray (Variables|CoolDown|GetInisial_CooldownQ) (Variables|CoolDown|GetInisial_CooldownW) (Variables|CoolDown|GetInisial_CooldownE) (Variables|CoolDown|GetInisial_CooldownR)))
  (Variables|Mana|SetInisial_Mana_Cost (Utilities|Array|MakeArray (Variables|Mana|GetSpell%201%20Cost) (Variables|Mana|GetSpell%202%20Cost) (Variables|Mana|GetSpell%203%20Cost) (Variables|Mana|GetSpell%204%20Cost)))
  (Utilities|Time|SetTimerbyEvent (EventDispatchers|CreateEvent :!event Custom|AutoRegen) 1.0 true))

(event Game|Damage|EventAnyDamage
  (params (Damage :type Float%20%28single-precision%29) (DamageType :type Damage%20Type%20Object%20Reference) (InstigatedBy :type Controller%20Object%20Reference) (DamageCauser :type Actor%20Object%20Reference))
  ;[1 0.02459 0.01199 0.5] Damaged Gestion
  (Variables|Health|SetDamage%20Taken Damage)
  (if (not (== DamageType "/Game/LeagueOfLegends/Character/Ability_Damage.Ability_Damage"))
    (bind _output_get (Variables|Health|SetHealth (- (Variables|Health|GetHealth) (- (Variables|Health|GetDamage%20Taken) (/ (Variables|Health|GetDamage%20Taken) (Variables|Statistiques|GetArmor))))))
    (Default|HealthBarUpdate (Variables|HUD|GetAs%20WBP%20Health%20Bar) (/ _output_get (Variables|Health|GetMaxHealth)))
    (if (!= (Utilities|GetClass self) "/Game/LeagueOfLegends/Champion/Dummy/BP_Dummy.BP_Dummy_C")
      (Default|UpdateLife (Variables|HUD|GetAs%20BP%20HUD%20LOL) (/ (Variables|Health|GetHealth) (Variables|Health|GetMaxHealth)) (Variables|Health|GetHealth))
      (if (<= (Variables|Health|GetHealth) 0.0)
        (CallFunction|Die)))))

(fn ConstructionScript)

(fn PostionforAttack
  (params (Range :type Float%20%28double-precision%29))
  (bind _enemilocation (Variables|AA|GetEnemiLocation))
  (bind _position (Variables|AA|GetPosition))
  (bind _returnvalue (- _enemilocation _position))
  (bind (_x _y) (Math|Vector|BreakVector _returnvalue))
  (bind _returnvalue_2 (Math|Vector|MakeVector _x _y 0.0))
  ;[0.4508 0.2831 0.01764] Calcul the position to make the enemy in range of attack whith a range
  (bind _output_get (Variables|AA|SetPositionForAttack (+ (* (Math|Float|Max(Float) (- (Math|Vector|VectorLength _returnvalue_2) (- Range 5e+01)) 0.0) (Math|Vector|Normalize _returnvalue_2)) (Variables|AA|GetPosition))))
  (return _output_get))

(fn RangeCheck
  (params (StartPosition :type Vector) (EndPosition :type Vector) (Range :type Float%20%28double-precision%29))
  (bind _output_get (Variables|AA|SetIsInRange (<= (Math|Vector|Distance(Vector) StartPosition EndPosition) Range)))
  (return _output_get))

(fn CanCasttheSpell?
  (params (SpellCost :type Float%20%28double-precision%29) (CoolDown :type Float%20%28double-precision%29) (Range :type Static%20Mesh%20Component%20Object%20Reference))
  (bind _manacurrent (Variables|Mana|GetManaCurrent))
  (bind _returnvalue (- _manacurrent SpellCost))
  (bind _returnvalue_2 (>= _returnvalue 0.0))
  (if (Math|Boolean|ANDBoolean (not (Variables|Spells|GetIsCastingASpell?)) _returnvalue_2 (== CoolDown 0.0))
    (if (Utilities|IsValid Range)
      (Rendering|SetVisibility Range false false))
    (return true false)
    (else
      (return false _returnvalue_2))))