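; HUD Blueprint for the League of Legends-style game, managing the player widget and the end screen.
; On BeginPlay it creates WBP_Player, hands it the player's BP_Character, binds to that character's death event and disables its own tick.
; Its events relay health, mana, rage animation and per-index or looped cooldown animations and resets to the widget.
; DeathScreen swaps the player widget for WBP_End.
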(event Custom|UpdateLife
  (params (InPercent :type Float%20%28single-precision%29) (CurrentHealth :type Float%20%28double-precision%29))
  (Default|UpdateHealth (Variables|Default|GetAs%20WBP%20Player) InPercent CurrentHealth))

(event Custom|UpdateMana
  (params (InPercent :type Float%20%28single-precision%29) (CurrentMana :type Float%20%28double-precision%29))
  (Default|UpdateMana (Variables|Default|GetAs%20WBP%20Player) InPercent CurrentMana))

(event Custom|DeathScreen
  (Widget|RemovefromParent (Variables|Default|GetWidget_HUD))
  (bind _returnvalue (UserInterface|CreateWidget "/Game/LeagueOfLegends/Widgets/WBP_End.WBP_End_C"))
  (UserInterface|Viewport|AddtoViewport _returnvalue 0))

(event Custom|CooldownSystem
  (params (index :type Integer))
  (Default|CooldownAnimation (Variables|Default|GetAs%20WBP%20Player) index)
  (Variables|Default|SetStart (Utilities|Time|GetGameTimeinSeconds)))

(event Custom|AllReset
  (params (index :type Integer))
  (for _index (range 0 index)
    (Default|CoolDownReset (Variables|Default|GetAs%20WBP%20Player) _index)))

(event Custom|Reset
  (params (index :type Integer))
  (Default|CoolDownReset (Variables|Default|GetAs%20WBP%20Player) index))

(event Custom|Rage
  (Default|RageAnimPlay (Variables|Default|GetAs%20WBP%20Player)))

(event EventBeginPlay
  (bind _asbp_character (Utilities|Casting|CastToBP_Character (Game|Player|GetPlayerPawn 0)))
  (bind _output_get (Variables|Default|SetAs%20BP%20Character _asbp_character))
  (EventDispatchers|BindEventtoOnCharacterDie _output_get (EventDispatchers|CreateEvent :!event Custom|DeathScreen))
  (bind _returnvalue (UserInterface|CreateWidget "/Game/LeagueOfLegends/Widgets/WBP_Player.WBP_Player_C" 0 0))
  (bind _output_get_2 (Variables|Default|SetWidget_HUD _returnvalue))
  (UserInterface|Viewport|AddtoViewport _output_get_2 0)
  (bind _aswbp_player (Utilities|Casting|CastToWBP_Player _output_get_2))
  (bind _output_get_3 (Variables|Default|SetAs%20WBP%20Player _aswbp_player))
  (Variables|/Game/LeagueOfLegends/Widgets/WBP_Player.WBP_Player_C|SetPlayer _output_get_3 (Variables|Default|GetAs%20BP%20Character))
  (Actor|Tick|SetActorTickEnabled false))

(event Collision|EventActorBeginOverlap
  (params (OtherActor :type Actor%20Object%20Reference)))

(fn ConstructionScript)