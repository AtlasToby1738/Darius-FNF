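; Homing turret projectile that damages the local player on contact.
; BeginPlay passes the target component to ProjectileMovement for homing and scales the Niagara effect's Size from Damage.
; Tick re-yaws the effect from the direction to the target, offset by the player's control yaw.
; The sphere overlap reacts only to player pawn 0, applying damage and destroying the projectile.
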(event OnComponentBeginOverlap(Sphere)
  (params (OverlappedComponent :type Primitive%20Component%20Object%20Reference) (OtherActor :type Actor%20Object%20Reference) (OtherComp :type Primitive%20Component%20Object%20Reference) (OtherBodyIndex :type Integer) (bFromSweep :type Boolean) (SweepResult :type Hit%20Result%20Structure%20%28by%20ref%29))
  (if (== OtherActor (Game|Player|GetPlayerPawn 0))
    (Game|Damage|ApplyDamage OtherActor (Variables|Default|GetDamage) 0 0 "/Script/Engine.DamageType")
    (Actor|DestroyActor)))

(event EventBeginPlay
  ;[0.01229 0.02029 0.02217] Set niagara Size with damage
  (Variables|/Script/Engine.ProjectileMovementComponent|SetHomingTargetComponent (Variables|Default|GetProjectileMovement) (Variables|Default|GetHoming%20Target%20Component))
  (Niagara|SetNiagaraVariable(Float) (Variables|Default|GetNiagara) "Size" (/ (Variables|Default|GetDamage) 5.0)))

(event EventTick
  (params (DeltaSeconds :type Float%20%28single-precision%29))
  ;[0.07819 0.1529 0.06848] Make face the player while chassing
  (Transformation|SetWorldRotation (Variables|Default|GetNiagara) (Math|Rotator|MakeRotator 0.0 0.0 (Utilities|Operators|Subtract (.Yaw (Math|Rotator|BreakRotator (Math|Rotator|FindLookatRotation (Transformation|GetActorLocation) (Transformation|GetWorldLocation (Variables|Default|GetHoming%20Target%20Component))))) (.yaw (Pawn|GetControlRotation (Game|Player|GetPlayerPawn 0) :!class /Script/Engine.Pawn)) 1.8e+02)) false false))

(fn ConstructionScript)