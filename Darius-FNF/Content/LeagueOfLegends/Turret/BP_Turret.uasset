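; BP_Turret is a League of Legends-style team turret that attacks the player pawn while it overlaps the turret's range sphere.
; On overlap it swaps the indicator material, plays a sound and, after a short delay, starts a looping timer spawning homing projectiles from a bone.
; Consecutive shots scale damage through a capped array index; end overlap by non-dummy actors resets timers and shot count.
; The construction script applies blue or red materials by team.
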(event OnComponentBeginOverlap(Sphere1)
  (params (OverlappedComponent :type Primitive%20Component%20Object%20Reference) (OtherActor :type Actor%20Object%20Reference) (OtherComp :type Primitive%20Component%20Object%20Reference) (OtherBodyIndex :type Integer) (bFromSweep :type Boolean) (SweepResult :type Hit%20Result%20Structure%20%28by%20ref%29))
  ;[0.01033 0.01161 0.01033] Take agro on collition with player
  (if (== OtherActor (Game|Player|GetPlayerPawn 0))
    (Utilities|FlowControl|DoOnce false
      (:Completed
        (Variables|Default|SetOverlapped%20Component (Actor|GetComponentbyClass OtherActor "/Script/Engine.SkeletalMeshComponent"))
        (Audio|PlaySound2D "/Game/LeagueOfLegends/Sound/Turret.Turret" 0.1 1.0 0.1 0 0)
        (Rendering|Material|SetMaterial (Variables|Default|GetSphere) 0 "/Game/LeagueOfLegends/Matrerials/MI_Turret_Triggered.MI_Turret_Triggered")
        (bind _returnvalue (Utilities|Time|SetTimerbyEvent (delegate Custom|Trigger) 0.2))
        (Variables|Default|SetTriggerTimer _returnvalue)))))

(event OnComponentEndOverlap(Sphere1)
  (params (OverlappedComponent :type Primitive%20Component%20Object%20Reference) (OtherActor :type Actor%20Object%20Reference) (OtherComp :type Primitive%20Component%20Object%20Reference) (OtherBodyIndex :type Integer))
  ;[0.15 0.15 0.15 0.5] Cancle everything exepted projectile when the player end overlap with the collider
  (if (!= (Utilities|GetClass OtherActor) "/Game/LeagueOfLegends/Champion/Dummy/BP_Dummy.BP_Dummy_C")
    (Rendering|Material|SetMaterial (Variables|Default|GetSphere) 0 "/Game/LeagueOfLegends/Matrerials/MI_Turret_Waiting.MI_Turret_Waiting")
    (CallFunction|ResetTower)
    (CallFunction|ResetTowerAttack)))

(event Custom|Trigger
  ;[0.6867 0.04092 0.03955] Fire projectile when the timer is over
  (Game|SpawnActorfromClass "/Game/LeagueOfLegends/Turret/BP_Turret_Projectil.BP_Turret_Projectil_C" (Math|Transform|MakeTransform (.location (Transformation|GetBoneTransform (Variables|Default|GetBlueTurret) "Break3_014" "RTS_World")) "0, 0, 0" "1.000000,1.000000,1.000000") "Undefined" "MultiplyWithRoot" 0 (Variables|Default|GetOverlapped%20Component) (* (Variables|Default|GetDamage) (Utilities|Array|Get(acopy) (Variables|Default|GetDamage%25) (Variables|Default|GetTowerShot))) 0)
  (Variables|Default|SetTowerShot (Math|Integer|Clamp(Integer) (+ (Variables|Default|GetTowerShot) 1) 0 3))
  (Utilities|FlowControl|DoOnce false
    (:Completed
      (bind _returnvalue (Utilities|Time|SetTimerbyEvent (delegate Custom|Trigger) (Variables|Default|GetAttaqueSpeed) true))
      (Variables|Default|SetAttackspeed _returnvalue))))

(event Custom|ResetTower
  ;[0.01033 0.01161 0.01033] Take agro on collition with player
  (Variables|Default|SetTowerShot 0)
  (Utilities|Time|ClearandInvalidateTimerbyHandle (Variables|Default|GetTriggerTimer))
  (Utilities|FlowControl|DoOnce false) ; enters at Reset
)

(event Custom|ResetTowerAttack
  ;[0.6867 0.04092 0.03955] Fire projectile when the timer is over
  (Utilities|Time|ClearandInvalidateTimerbyHandle (Variables|Default|GetAttackspeed))
  (Utilities|FlowControl|DoOnce false) ; enters at Reset
)

(fn ConstructionScript
  (bind _blueturret (Variables|Default|GetBlueTurret))
  (if (Variables|Default|GetBlueTeam?)
    (for _index (range 0 2)
      (Rendering|Material|SetMaterial _blueturret _index "/Game/LeagueOfLegends/Turret/Materials/M_Blue_Turret.M_Blue_Turret"))
    (else
      (for _index_2 (range 0 2)
        (Rendering|Material|SetMaterial _blueturret _index_2 "/Game/LeagueOfLegends/Turret/Materials/M_Red_Turret.M_Red_Turret")))))