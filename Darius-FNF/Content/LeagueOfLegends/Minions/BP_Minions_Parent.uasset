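; BP_Minions_Parent is the base Blueprint for League of Legends-style minions, adding out-of-combat health recovery to the behavior it inherits.
; AnyDamage runs the parent damage handling, then a retriggerable delay restarts on every hit, so Health snaps back to MaxHealth only after a few seconds without damage.
; A debug "heal" string prints on reset, while BeginPlay and construction only call the parent.
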(event EventBeginPlay
  (|CallParentFunction))

(event Collision|EventActorBeginOverlap
  (params (OtherActor :type Actor%20Object%20Reference))
  (|CallParentFunction OtherActor) ; Ce nœud est désactivé et ne sera pas appelé.\nFaites glisser les broches pour générer des fonctionnalités.
)

(event EventTick
  (params (DeltaSeconds :type Float%20%28single-precision%29))
  (|CallParentFunction DeltaSeconds) ; Ce nœud est désactivé et ne sera pas appelé.\nFaites glisser les broches pour générer des fonctionnalités.
)

(event Game|Damage|EventAnyDamage
  (params (Damage :type Float%20%28single-precision%29) (DamageType :type Damage%20Type%20Object%20Reference) (InstigatedBy :type Controller%20Object%20Reference) (DamageCauser :type Actor%20Object%20Reference))
  (|CallParentFunction Damage DamageType InstigatedBy DamageCauser)
  (Utilities|FlowControl|RetriggerableDelay 5.0)
  (Variables|Default|SetHealth (Variables|Default|GetMaxHealth))
  (Development|PrintString "heal"))

(fn ConstructionScript
  (|CallParentFunction))