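; BP_Speed_Boss is a boss Blueprint that changes the game manager's movement duration as its special effect.
; It caches BP_GameManager on BeginPlay, and its Effect event writes NewSpeed into the manager's MovementDuration.
; When damage leaves Health at 50 or below, a DoOnce shortens the duration and calls the parent Effect; death restores a longer duration before the parent Die logic.
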(event EventEffect
  ;[0.03955 0.6584 0] Effect *2 SpawnRate
  (Variables|/Game/FridayNightFunkin/Blueprints/BP_GameManager.BP_GameManager_C|SetMovement%20Duration (Variables|Default|GetManager) (Variables|Default|GetNewSpeed)))

(event EventBeginPlay
  ;[0.06125 0.1529 0.2423] BeginPlay Parent + get GameManger
  (|CallParentFunction)
  (bind _returnvalue (Actor|GetActorOfClass "/Game/FridayNightFunkin/Blueprints/BP_GameManager.BP_GameManager_C"))
  (Variables|Default|SetManager _returnvalue))

(event Game|Damage|EventAnyDamage
  (params (Damage :type Float%20%28single-precision%29) (DamageType :type Damage%20Type%20Object%20Reference) (InstigatedBy :type Controller%20Object%20Reference) (DamageCauser :type Actor%20Object%20Reference))
  ;[0.2122 0.06301 0.01033] Damage to use the effect one time when the hp is less than 50 and 25 hp
  (|CallParentFunction Damage DamageType InstigatedBy DamageCauser)
  (if (<= (Variables|Default|GetHealth) 5e+01)
    (Utilities|FlowControl|DoOnce false
      (:Completed
        (Variables|Default|SetNewSpeed 0.6)
        (CallFunction|Effect)
        (|CallParentFunction)))))

(event EventDie
  ;[1 1 1 0.5] Die with reset
  (Variables|Default|SetNewSpeed 0.9)
  (CallFunction|Effect)
  (|CallParentFunction))

(fn ConstructionScript
  (|CallParentFunction))