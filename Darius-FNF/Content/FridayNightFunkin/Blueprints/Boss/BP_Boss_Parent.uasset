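; BP_Boss_Parent is the base Blueprint for bosses, handling health, the boss health bar and death.
; On BeginPlay it resets health, takes the WBP_BossBar from its widget component and applies the boss's image and color.
; Damage updates the bar and health, and once the bar's percent drops below a threshold it fires OnBossKill, bound to destroy the actor.
; A separate Effect event plays a 2D sound.
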(event Custom|Effect
  ;[0.3005 0 0.5521 0.5] Boss's effect
  (Audio|SpawnSound2D (Variables|Default|GetSound) 1.0 1.0 0.0 0))

(event Custom|Die
  ;[0.0648 0.1441 0.2122] BeginPlay
  (Actor|DestroyActor))

(event EventBeginPlay
  ;[0.0648 0.1441 0.2122] BeginPlay
  (Variables|Default|SetHealth (Variables|Default|GetMaxHealth))
  (bind _aswbp_boss_bar (Utilities|Casting|CastToWBP_BossBar (UserInterface|GetWidget (Variables|Default|GetWidget))))
  (bind _output_get (Variables|Default|SetWBP%20Boss%20Bar _aswbp_boss_bar))
  (Default|SetPreset _output_get (Variables|Default|GetImage) (Variables|Default|GetColor))
  (EventDispatchers|BindEventtoOnBossKill (delegate Custom|Die)))

(event Game|Damage|EventAnyDamage
  (params (Damage :type Float%20%28single-precision%29) (DamageType :type Damage%20Type%20Object%20Reference) (InstigatedBy :type Controller%20Object%20Reference) (DamageCauser :type Actor%20Object%20Reference))
  (bind _wbp_boss_bar (Variables|Default|GetWBP%20Boss%20Bar))
  ;[1 0.15 0.15 0.5] Take Damage
  (Default|UpdateLife _wbp_boss_bar Damage)
  (Variables|Default|SetHealth (- (Variables|Default|GetHealth) Damage))
  (if (< (Variables|/Script/UMG.ProgressBar|GetPercent (Variables|/Game/FridayNightFunkin/Widgets/WBP_BossBar.WBP_BossBar_C|GetHealthBar _wbp_boss_bar)) (Variables|Default|GetThreshOld))
    (Default|CallOnBossKill)))

(fn ConstructionScript)