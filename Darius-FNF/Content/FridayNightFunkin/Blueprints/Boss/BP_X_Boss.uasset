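; BP_X_Boss is a boss Blueprint in the Friday Night Funkin game that switches on the X probability mechanic through the game manager.
; On BeginPlay it caches the BP_GameManager actor and fires Effect, whose FlipFlop sets the manager's X flag and runs the parent effect.
; Die fires Effect again so the FlipFlop's second branch clears the flag, then runs the parent death logic.
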(event EventEffect
  (bind _manager (Variables|Default|GetManager))
  ;[0.15 0.15 0.15 0.5] Effet qui active le boolean pour activer la proba des X
  (Utilities|FlowControl|FlipFlop
    (:A
      (Variables|/Game/FridayNightFunkin/Blueprints/BP_GameManager.BP_GameManager_C|SetX? _manager true)
      (|CallParentFunction))
    (:B
      (Variables|/Game/FridayNightFunkin/Blueprints/BP_GameManager.BP_GameManager_C|SetX? _manager false))))

(event EventBeginPlay
  ;[0.06125 0.1529 0.2423] BeginPlay Parent + get GameManger
  (|CallParentFunction)
  (bind _returnvalue (Actor|GetActorOfClass "/Game/FridayNightFunkin/Blueprints/BP_GameManager.BP_GameManager_C"))
  (Variables|Default|SetManager _returnvalue)
  (CallFunction|Effect))

(event EventDie
  ;[0.5333 0.2664 0.2664] Die and active the effect to cancle
  (CallFunction|Effect)
  (|CallParentFunction))

(fn ConstructionScript
  (|CallParentFunction))