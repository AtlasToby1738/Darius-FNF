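; Fog boss that extends a parent boss Blueprint with a screen blur effect on the player's HUD widget.
; BeginPlay caches the widget from BP_HUD, and the Effect override plays its blur animation alongside the parent effect.
; Effect fires once when damage leaves health at or below half, and again on death to reset it.
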(event EventBeginPlay
  ;[1 0.03955 0.03955] BeginPlay To get HUD and Parent BeginPlay
  (|CallParentFunction)
  (bind _asbp_hud (Utilities|Casting|CastToBP_HUD (HUD|GetHUD (Game|GetPlayerController 0))))
  (Variables|Default|SetWBP%20HUD (Variables|/Game/FridayNightFunkin/Blueprints/Character/BP_HUD.BP_HUD_C|GetWBP_HUD _asbp_hud)))

(event EventEffect
  ;[0.1878 0.08438 0.02956] Effect Prock
  (Default|BlurAnimation (Variables|Default|GetWBP%20HUD))
  (|CallParentFunction))

(event Game|Damage|EventAnyDamage
  (params (Damage :type Float%20%28single-precision%29) (DamageType :type Damage%20Type%20Object%20Reference) (InstigatedBy :type Controller%20Object%20Reference) (DamageCauser :type Actor%20Object%20Reference))
  ;[1 0.15 0.15 0.5] Comment
  (|CallParentFunction Damage DamageType InstigatedBy DamageCauser)
  (if (<= (Variables|Default|GetHealth) (/ (Variables|Default|GetMaxHealth) 2.0))
    (Utilities|FlowControl|DoOnce false
      (:Completed
        (CallFunction|Effect)))))

(event EventDie
  ;[0.15 0.15 0.15 0.5] Die and effect to reset
  (CallFunction|Effect)
  (|CallParentFunction))

(fn ConstructionScript
  (|CallParentFunction))