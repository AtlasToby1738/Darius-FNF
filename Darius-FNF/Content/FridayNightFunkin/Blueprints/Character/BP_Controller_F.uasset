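; Player controller for the Friday Night Funkin-style rhythm game, handling arrow input, score, life and pause.
; Each of four direction inputs scans spawned arrows by world height, then hits the chosen one or calls Fail.
; Score events refill the lifebar through BP_HUD, or damage the boss when it is full outside tutorials.
; Fail drains life until LoseGame pauses play; the pause menu is blocked on the FRIDAY level.
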(event Custom|CheckForArrows
  (params (Direction :type E_Direction%20Enum :default "NewEnumerator0"))
  ;[1 0 1 0.5] Arrow System
  (bind _outactors (Actor|GetAllActorsOfClass "/Game/FridayNightFunkin/Blueprints/Arrows/Blueprints/BP_Arrows_Parents.BP_Arrows_Parents_C"))
  (bind _output_get (Variables|Arrow|SetAllArrows _outactors))
  (if (Utilities|Array|IsEmpty _output_get)
    (CallFunction|Fail)
    (else
      (for _array_element (Variables|Arrow|GetAllArrows)
        (if (not (Variables|/Game/FridayNightFunkin/Blueprints/Arrows/Blueprints/BP_Arrows_Parents.BP_Arrows_Parents_C|GetExemple%20? _array_element))
          (Utilities|Array|Add (Variables|Arrow|GetTrueArrowTable) _array_element)))
      (for _array_element_2 (Variables|Arrow|GetTrueArrowTable)
        (Utilities|IsValid _array_element_2
          (:Is%20Valid
            (if (and (<= (.z (Transformation|GetWorldLocation (Variables|/Game/FridayNightFunkin/Blueprints/Arrows/Blueprints/BP_Arrows_Parents.BP_Arrows_Parents_C|GetDefaultSceneRoot _array_element_2))) 7.5e+02) (or (>= (Variables|Arrow|GetHighestArrowZ) 6.5e+02) (> (.z (Transformation|GetWorldLocation (Variables|/Game/FridayNightFunkin/Blueprints/Arrows/Blueprints/BP_Arrows_Parents.BP_Arrows_Parents_C|GetDefaultSceneRoot _array_element_2))) (Variables|Arrow|GetHighestArrowZ))))
              (Variables|Arrow|SetHighestArrow _array_element_2)
              (Variables|Arrow|SetHighestArrowZ (.z (Transformation|GetWorldLocation (Variables|/Game/FridayNightFunkin/Blueprints/Arrows/Blueprints/BP_Arrows_Parents.BP_Arrows_Parents_C|GetDefaultSceneRoot _array_element_2))))))))
      (Utilities|IsValid (Variables|Arrow|GetHighestArrow)
        (:Is%20Valid
          (if (and (Utilities|Enum|Equal(Enum) Direction (Variables|/Game/FridayNightFunkin/Blueprints/Arrows/Blueprints/BP_Arrows_Parents.BP_Arrows_Parents_C|GetEnumDirection (Variables|Arrow|GetHighestArrow))) (>= (Variables|Arrow|GetHighestArrowZ) (Variables|Arrow|GetHighMin)))
            (Default|ArrowGotPressed (Variables|Arrow|GetHighestArrow))
            (else
              (CallFunction|Fail)
              (Default|ArrowMiss (Variables|Arrow|GetHighestArrow))))
          (Variables|Arrow|SetHighestArrowZ 0.0))))))

(event Custom|Attack%20Boss
  (params (BaseDamage :type Float%20%28single-precision%29))
  ;[1 0.15 0.15 0.5] Damage boss
  (bind _returnvalue (Actor|GetActorOfClass "/Game/FridayNightFunkin/Blueprints/Boss/BP_Boss_Parent.BP_Boss_Parent_C"))
  (Game|Damage|ApplyDamage _returnvalue BaseDamage 0 0))

(event Custom|Fail
  (bind _bp_hud (Variables|Menu|GetBP%20HUD))
  (bind _wbp_hud (Variables|/Game/FridayNightFunkin/Blueprints/Character/BP_HUD.BP_HUD_C|GetWBP_HUD _bp_hud))
  (bind _lifebar (Variables|/Game/FridayNightFunkin/Widgets/WBP_HUD_Friday.WBP_HUD_Friday_C|GetLifebar _wbp_hud))
  (bind _percent (Variables|/Script/UMG.ProgressBar|GetPercent _lifebar))
  ;[1 0.6063 0.1765 0.5] Score Update
  (if (<= _percent 0.1)
    (CallFunction|LoseGame)
    (else
      (Default|SetLife (Variables|/Game/FridayNightFunkin/Blueprints/Character/BP_HUD.BP_HUD_C|GetWBP_HUD (Variables|Menu|GetBP%20HUD)) (- _percent 0.1))
      (Audio|SpawnSound2D "/Game/FridayNightFunkin/Sound/Miss/SC_Miss.SC_Miss" 1.0 1.0 0.0 0))))

(event Custom|Score
  (params (Score :type Float%20%28double-precision%29) (IntexHit :type Integer))
  (bind _bp_hud (Variables|Menu|GetBP%20HUD))
  (bind _wbp_hud (Variables|/Game/FridayNightFunkin/Blueprints/Character/BP_HUD.BP_HUD_C|GetWBP_HUD _bp_hud))
  (bind _lifebar (Variables|/Game/FridayNightFunkin/Widgets/WBP_HUD_Friday.WBP_HUD_Friday_C|GetLifebar _wbp_hud))
  (bind _percent (Variables|/Script/UMG.ProgressBar|GetPercent _lifebar))
  ;[1 0.6063 0.1765 0.5] Score Update
  (bind _output_get (Variables|Menu|SetCurrentScore (+ Score (Variables|Menu|GetCurrentScore))))
  (Default|SetScore (Variables|/Game/FridayNightFunkin/Blueprints/Character/BP_HUD.BP_HUD_C|GetWBP_HUD (Variables|Menu|GetBP%20HUD)) (Utilities|Text|ToText(Float) _output_get "HalfToEven"))
  (Variables|Menu|SetIndexHit IntexHit)
  (Default|SpawnScore (Variables|/Game/FridayNightFunkin/Blueprints/Character/BP_HUD.BP_HUD_C|GetWBP_HUD (Variables|Menu|GetBP%20HUD)) (Variables|Menu|GetIndexHit))
  (if (and (not (Variables|/Game/FridayNightFunkin/Blueprints/Character/BP_HUD.BP_HUD_C|GetTutorial? (Variables|Menu|GetBP%20HUD))) (>= _percent 1.0))
    (CallFunction|AttackBoss (Utilities|Array|Get(acopy) (Variables|Damage|GetDamageTable) (Variables|Menu|GetIndexHit)))
    (Default|SpawnDamage (Variables|/Game/FridayNightFunkin/Blueprints/Character/BP_HUD.BP_HUD_C|GetWBP_HUD (Variables|Menu|GetBP%20HUD)) (Variables|Menu|GetIndexHit))
    (else
      (Default|SetLife (Variables|/Game/FridayNightFunkin/Blueprints/Character/BP_HUD.BP_HUD_C|GetWBP_HUD (Variables|Menu|GetBP%20HUD)) (+ _percent 0.1)))))

(event Custom|LoseGame
  ;[0.15 0.15 0.15 0.5] Lose Game
  (Default|CallEndGame)
  (Audio|SpawnSound2D "/Game/FridayNightFunkin/Sound/Miss/Death.Death" 1.0 1.0 0.0 0)
  (Game|SetGamePaused true))

(event Custom|GameStart
  (bind _returnvalue (Game|GetPlayerController 0))
  ;[0.05613 0.1413 0.2232] Game launch system
  (Input|AddMappingContext (PlayerController|LocalPlayerSubsystems|GetEnhancedInputLocalPlayerSubsystem _returnvalue) "/Game/FridayNightFunkin/Inputs/IMC_Friday.IMC_Friday" 0 "(bIgnoreAllPressedKeysUntilRelease=True,bForceImmediately=False,bNotifyUserSettings=False)")
  (Input|SetInputModeGameOnly _returnvalue false)
  (Variables|/Script/Engine.PlayerController|SetbShowMouseCursor _returnvalue false)
  (bind _asbp_hud (Utilities|Casting|CastToBP_HUD (HUD|GetHUD)))
  (Variables|Menu|SetBP%20HUD _asbp_hud))

(event Input|EnhancedActionEvents|EnhancedInputActionAI_Pause
  (params (ActionValue :type Boolean) (ElapsedSeconds :type Float%20%28double-precision%29) (TriggeredSeconds :type Float%20%28double-precision%29) (InputAction :type Input%20Action%20Object%20Reference :default "/Game/LeagueOfLegends/Input/AI_Pause.AI_Pause"))
  (bind _returnvalue (Game|GetPlayerController 0))
  ;[1 1 1 0.5] Pause Menu
  (bind _returnvalue_2 (Game|GetCurrentLevelName true))
  (if (not (Utilities|Enum|Equal(Enum) _returnvalue_2 "FRIDAY"))
    (Default|CallEDTest)
    (Utilities|FlowControl|DelayUntilNextTick)
    (Game|SetGamePaused true)
    (bind _returnvalue_3 (UserInterface|CreateWidget "/Game/FridayNightFunkin/Widgets/WBP_Pause_FNF.WBP_Pause_FNF_C"))
    (bind _output_get (Variables|Menu|SetWBP_Pause _returnvalue_3))
    (UserInterface|Viewport|AddtoViewport _output_get 0)
    (Input|SetInputModeGameandUI _returnvalue _output_get "DoNotLock" true false)
    (Variables|/Script/Engine.PlayerController|SetbShowMouseCursor _returnvalue true)))

(event Input|EnhancedActionEvents|EnhancedInputActionAI_Up
  (params (ActionValue :type Boolean) (ElapsedSeconds :type Float%20%28double-precision%29) (TriggeredSeconds :type Float%20%28double-precision%29) (InputAction :type Input%20Action%20Object%20Reference :default "/Game/FridayNightFunkin/Inputs/AI_Up.AI_Up"))
  ;[1 0 0 0.5] Inputs
  (:Started
    (Variables|Arrow|SetAction%20Value ActionValue)
    (bind _output_get (Variables|Arrow|SetDirectionEnum "NewEnumerator2"))
    (CallFunction|CheckforArrows _output_get))
  (:Ongoing
    (Variables|Arrow|SetTriggered%20Seconds ElapsedSeconds))
  (:Canceled
    (Variables|Arrow|SetAction%20Value false :!label _label)
    (Variables|Arrow|SetTriggered%20Seconds 0.0))
  (:Completed
    (goto _label)))

(event Input|EnhancedActionEvents|EnhancedInputActionAI_Left
  (params (ActionValue :type Boolean) (ElapsedSeconds :type Float%20%28double-precision%29) (TriggeredSeconds :type Float%20%28double-precision%29) (InputAction :type Input%20Action%20Object%20Reference :default "/Game/FridayNightFunkin/Inputs/AI_Left.AI_Left"))
  ;[1 0 0 0.5] Inputs
  (:Started
    (Variables|Arrow|SetAction%20Value ActionValue)
    (bind _output_get (Variables|Arrow|SetDirectionEnum "NewEnumerator0"))
    (CallFunction|CheckforArrows _output_get))
  (:Ongoing
    (Variables|Arrow|SetTriggered%20Seconds ElapsedSeconds))
  (:Canceled
    (Variables|Arrow|SetAction%20Value false :!label _label)
    (Variables|Arrow|SetTriggered%20Seconds 0.0))
  (:Completed
    (goto _label)))

(event Input|EnhancedActionEvents|EnhancedInputActionAI_Right
  (params (ActionValue :type Boolean) (ElapsedSeconds :type Float%20%28double-precision%29) (TriggeredSeconds :type Float%20%28double-precision%29) (InputAction :type Input%20Action%20Object%20Reference :default "/Game/FridayNightFunkin/Inputs/AI_Right.AI_Right"))
  ;[1 0 0 0.5] Inputs
  (:Started
    (Variables|Arrow|SetAction%20Value ActionValue)
    (bind _output_get (Variables|Arrow|SetDirectionEnum "NewEnumerator3"))
    (CallFunction|CheckforArrows _output_get))
  (:Ongoing
    (Variables|Arrow|SetTriggered%20Seconds ElapsedSeconds))
  (:Canceled
    (Variables|Arrow|SetAction%20Value false :!label _label)
    (Variables|Arrow|SetTriggered%20Seconds 0.0))
  (:Completed
    (goto _label)))

(event Input|EnhancedActionEvents|EnhancedInputActionAI_Down
  (params (ActionValue :type Boolean) (ElapsedSeconds :type Float%20%28double-precision%29) (TriggeredSeconds :type Float%20%28double-precision%29) (InputAction :type Input%20Action%20Object%20Reference :default "/Game/FridayNightFunkin/Inputs/AI_Down.AI_Down"))
  ;[1 0 0 0.5] Inputs
  (:Started
    (Variables|Arrow|SetAction%20Value ActionValue)
    (bind _output_get (Variables|Arrow|SetDirectionEnum "NewEnumerator1"))
    (CallFunction|CheckforArrows _output_get))
  (:Ongoing
    (Variables|Arrow|SetTriggered%20Seconds ElapsedSeconds))
  (:Canceled
    (Variables|Arrow|SetAction%20Value false :!label _label)
    (Variables|Arrow|SetTriggered%20Seconds 0.0))
  (:Completed
    (goto _label)))

(event EventTick
  (params (DeltaSeconds :type Float%20%28single-precision%29))
  ;[1 1 1] Tick for the hold info
)

(fn ConstructionScript)