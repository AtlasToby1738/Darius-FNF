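; Game manager for a Friday Night Funkin' rhythm level, handling countdown, music, arrow spawning, bosses and pause toggling.
; After the countdown, tutorial mode plays song and voice tracks while Tick spawns preset arrows ahead by their travel time, broadcasting when the song ends.
; Otherwise, infinite mode spawns random arrows on a looping timer and a random boss, replaced whenever destroyed.
; Both modes share one spawn path for standard and hold arrows.
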(event Custom|SpawnArrow
  ;[0 0 1] Spawn Random Arrows With a Timer
  (if (>= (Utilities|Time|GetGameTimeinSeconds) (+ (Variables|Spawn|GetTime%20Spawn) (Variables|Hold|GetHold%20Duration)))
    (Utilities|FlowControl|Delay 0.125)
    (bind _output_get (Variables|Spawn|SetArrowSelection (Math|Random|RandomIntegerinRange 0 4)))
    (if (not (== _output_get 4))
      (CallFunction|SpawnArrowfromPresset (- (Utilities|Time|GetGameTimeinSeconds) (Variables|Game|GetStartTimer)) (/ (Utilities|Array|Get(acopy) (Variables|Hold|GetTileOption) (Math|Random|RandomIntegerinRange (select (== (Utilities|Array|Get(acopy) (Variables|Spawn|GetArrowClassTab) _output_get) "/Game/FridayNightFunkin/Blueprints/Arrows/Blueprints/Childs/Hold/BP_Arrow_Hold.BP_Arrow_Hold_C") 1 0) (select (== (Utilities|Array|Get(acopy) (Variables|Spawn|GetArrowClassTab) _output_get) "/Game/FridayNightFunkin/Blueprints/Arrows/Blueprints/Childs/Hold/BP_Arrow_Hold.BP_Arrow_Hold_C") 3 0))) 8.0) (Utilities|Array|Get(acopy) (Variables|Hold|GetTileOption) (Math|Random|RandomIntegerinRange (select (== (Utilities|Array|Get(acopy) (Variables|Spawn|GetArrowClassTab) _output_get) "/Game/FridayNightFunkin/Blueprints/Arrows/Blueprints/Childs/Hold/BP_Arrow_Hold.BP_Arrow_Hold_C") 1 0) (select (== (Utilities|Array|Get(acopy) (Variables|Spawn|GetArrowClassTab) _output_get) "/Game/FridayNightFunkin/Blueprints/Arrows/Blueprints/Childs/Hold/BP_Arrow_Hold.BP_Arrow_Hold_C") 3 0))) (Variables|Spawn|GetExemple?) (Utilities|Select :Index (Math|Random|RandomIntegerinRange 0 3) :Option%200 "NewEnumerator0" :Option%201 "NewEnumerator1" :Option%202 "NewEnumerator2" :Option%203 "NewEnumerator3") (Variables|Spawn|GetMovement%20Duration) (select (== (Utilities|Array|Get(acopy) (Variables|Spawn|GetArrowClassTab) _output_get) "/Game/FridayNightFunkin/Blueprints/Arrows/Blueprints/Childs/Hold/BP_Arrow_Hold.BP_Arrow_Hold_C") "NewEnumerator1" "NewEnumerator0")))))

(event Custom|Countdown
  ;[0.05781 0.117 0.1651] Start The Game
  (bind _returnvalue (Audio|SpawnSound2D "/Game/FridayNightFunkin/Sound/Start/SC_Countdown.SC_Countdown" 1.0 1.0 0.0 0))
  (bind _output_get (Variables|Default|SetCD _returnvalue))
  (EventDispatchers|BindEventtoOnAudioFinished _output_get (delegate Custom|GameMode)))

(event Custom|An%20Other%20One
  (params (DestroyedActor :type Actor%20Object%20Reference))
  ;[0.0137 0.7454 0.4179] BossSpawn System
  (CallFunction|SpawnBoss))

(event Custom|InfinityLoop
  ;[0 0 1] Spawn Random Arrows With a Timer
  (bind _output_get (Variables|Game|SetIntrumental "/Game/FridayNightFunkin/Levels/Loop/Inst__mp3cut_net_.Inst__mp3cut_net_"))
  (bind _returnvalue (Audio|SpawnSound2D _output_get 0.3 1.0 0.0 0))
  (Variables|Default|SetIntrumentalMusic _returnvalue)
  (Utilities|FlowControl|Delay 0.0)
  (Utilities|Time|SetTimerbyEvent (delegate Custom|SpawnArrow) (Variables|Spawn|GetRythme) true))

(event Custom|Tutorial
  (bind _levelpresset (Variables|Game|GetLevelPresset))
  ;[0.6038 0.2232 0.9911] Music
  (Variables|Game|SetStartTimer (Utilities|Time|GetGameTimeinSeconds))
  ;;[0.0137 0.7529 0.4233] Set the Bool Array With the Length of the Presset
  (Utilities|Array|Resize (Variables|Spawn|GetArrowSpanned?) (Utilities|Array|Length (Variables|/Game/FridayNightFunkin/Levels/BP_LevelPreset.BP_LevelPreset_C|GetStructure _levelpresset)))
  (Actor|Tick|SetActorTickEnabled true)
  (switch name (Variables|/Game/FridayNightFunkin/Levels/BP_LevelPreset.BP_LevelPreset_C|GetName _levelpresset)
    (:Tutorial
      (Utilities|FlowControl|Sequence
        (:then_0
          (bind _returnvalue (Audio|SpawnSound2D (Variables|Game|GetIntrumental) 1.0 1.0 0.0 0))
          (bind _output_get (Variables|Default|SetIntrumentalMusic _returnvalue))
          (EventDispatchers|BindEventtoOnAudioFinished _output_get (delegate Custom|GameEnd)))
        (:then_1
          (bind _returnvalue_2 (Audio|SpawnSound2D (Variables|Game|GetPlayerVoice) 1.0 1.0 0.0 0))
          (Variables|Default|SetPlayerVoiceMusic _returnvalue_2))
        (:then_2
          (bind _returnvalue_3 (Audio|SpawnSound2D (Variables|Game|GetSecondVoice) 1.0 1.0 0.0 0))
          (Variables|Default|SetSecondVoiceMusic _returnvalue_3))))
    (:Teste
      (bind _output_get_2 (Variables|Game|SetIntrumental "/Game/FridayNightFunkin/Levels/Test/Marjolina_spotdown_org.Marjolina_spotdown_org"))
      (Audio|SpawnSound2D _output_get_2 0.3 1.0 0.0 0))))

(event Custom|SpawnSwitch
  (params (Selection :type E_ArrowType%20Enum :default "NewEnumerator0"))
  ;[0.5 0 0.5 0.5] Spawn Arrow System
  (switch Utilities|FlowControl|Switch|SwitchonE_ArrowType Selection
    (:NewEnumerator0
      (CallFunction|SpawnStandard (Variables|Spawn|GetSpawnLocation) (Variables|Spawn|GetDirection) (Variables|Spawn|GetTimeline%20Mult) (Variables|Spawn|GetExemple?) (Variables|Spawn|GetTime%20Spawn) (Variables|Game|GetStartTimer) (Variables|Spawn|GetX?)))
    (:NewEnumerator1
      (CallFunction|SpawnHold (Variables|Spawn|GetSpawnLocation) (Variables|Hold|GetHold%20Duration) (Variables|Hold|GetTileHoldDuration) (Variables|Spawn|GetDirection) (Variables|Spawn|GetTimeline%20Mult) (Variables|Spawn|GetExemple?) (Variables|Spawn|GetTime%20Spawn) (Variables|Game|GetStartTimer)))))

(event Custom|GameEnd
  ;[0.6038 0.2232 0.9911] Music
  (Default|CallOnTutorialEnded))

(event Custom|Spawn%20Boss
  ;[0.0137 0.7454 0.4179] BossSpawn System
  (bind _output_get (Variables|Boss|SetNewindex (Math|Random|RandomIntegerinRange 0 2)))
  (if (== _output_get (Variables|Boss|GetBossIndex))
    (Variables|Boss|SetBossIndex (Utilities|Select :Index (Variables|Boss|GetNewindex) :Option%200 1 :Option%201 2 :Option%202 0))
    (else
      (Variables|Boss|SetBossIndex (Variables|Boss|GetNewindex))))
  (bind _returnvalue (Game|SpawnActorfromClass (Utilities|Array|Get(acopy) (Variables|Boss|GetBossArray) (Variables|Boss|GetNewindex)) (Variables|Boss|GetBossSpawn) "Undefined" "MultiplyWithRoot" 0 0))
  (Game|BindEventtoOnDestroyed _returnvalue (delegate Custom|An%20Other%20One)))

(event Custom|GameMode
  ;[0.05781 0.117 0.1651] Start The Game
  (Variables|Game|GetTutorial?
    (:then
      (CallFunction|Tutorial))
    (:else
      (CallFunction|InfinityLoop)
      (CallFunction|SpawnBoss))))

(event Custom|SpawnArrowFromPresset
  (params (TimeSpawn :type Float%20%28double-precision%29) (HoldDuration :type Float%20%28double-precision%29) (TileHoldDuration :type Float%20%28double-precision%29) (Exemple? :type Boolean) (Direction :type E_Direction%20Enum :default "NewEnumerator0") (MovementDuration :type Float%20%28double-precision%29) (Index :type E_ArrowType%20Enum :default "NewEnumerator0"))
  ;[0.5 0 0.5 0.5] Spawn Arrow System
  (Variables|Spawn|SetTime%20Spawn TimeSpawn)
  (Variables|Hold|SetHold%20Duration HoldDuration)
  (Variables|Hold|SetTileHoldDuration TileHoldDuration)
  (Variables|Spawn|SetExemple? Exemple?)
  (Variables|Spawn|SetDirection Direction)
  (Variables|Spawn|SetTimeline%20Mult MovementDuration)
  (Variables|Spawn|SetArrowType Index)
  (if (Variables|Spawn|GetExemple?)
    (Variables|Spawn|SetSpawnLocation (Utilities|Array|Get(acopy) (Variables|Spawn|GetSpawnPointForExemple) (Utilities|Select :Index (Variables|Spawn|GetDirection) :NewEnumerator0 0 :NewEnumerator1 1 :NewEnumerator2 2 :NewEnumerator3 3)))
    (else
      (Variables|Spawn|SetSpawnLocation (Utilities|Array|Get(acopy) (Variables|Spawn|GetSpawnPointForTrueOne) (Utilities|Select :Index (Variables|Spawn|GetDirection) :NewEnumerator0 0 :NewEnumerator1 1 :NewEnumerator2 2 :NewEnumerator3 3)))))
  (CallFunction|SpawnSwitch (Variables|Spawn|GetArrowType))
  (Math|Integer|IncrementInt (Variables|Spawn|GetArrowIndex)))

(event Custom|TimeSet
  (bind _intrumentalmusic (Variables|Default|GetIntrumentalMusic))
  (bind _intrumentalmusic_2 (Variables|Default|GetIntrumentalMusic))
  (bind _intrumental (Variables|Game|GetIntrumental))
  ;[1 1 1] Pause
  (Variables|Game|GetTutorial?
    (:then
      (Utilities|FlowControl|FlipFlop
        (:A
          (Utilities|IsValid _intrumentalmusic
            (:Is%20Valid
              (Class|AudioComponent|SetPaused (Variables|Default|GetIntrumentalMusic) true)
              (Class|AudioComponent|SetPaused (Variables|Default|GetPlayerVoiceMusic) true)
              (Class|AudioComponent|SetPaused (Variables|Default|GetSecondVoiceMusic) true)
              (Actor|Tick|SetActorTickEnabled false))))
        (:B
          (Utilities|IsValid _intrumentalmusic
            (:Is%20Valid
              (Class|AudioComponent|SetPaused (Variables|Default|GetIntrumentalMusic) false)
              (Class|AudioComponent|SetPaused (Variables|Default|GetPlayerVoiceMusic) false)
              (Class|AudioComponent|SetPaused (Variables|Default|GetSecondVoiceMusic) false)
              (Actor|Tick|SetActorTickEnabled true))))))
    (:else
      (Utilities|FlowControl|FlipFlop
        (:A
          (Utilities|IsValid _intrumental
            (:Is%20Valid
              (Utilities|FlowControl|DelayUntilNextTick)
              (Class|AudioComponent|SetPaused _intrumentalmusic_2 true))))
        (:B
          (Utilities|IsValid _intrumental
            (:Is%20Valid
              (Class|AudioComponent|SetPaused _intrumentalmusic_2 false))))))))

(event Custom|SpawnStandard
  (params (Spawn%20Transform%20Location :type Vector) (EnumDirection :type E_Direction%20Enum :default "NewEnumerator0") (TimelineMult :type Float%20%28double-precision%29) (Exemple%20? :type Boolean) (TimeSpawn :type Float%20%28double-precision%29) (Start%20Timer :type Float%20%28double-precision%29) (ChanceX :type Boolean))
  ;[0.5 0 0.5 0.5] Spawn Arrow System
  (Game|SpawnActorfromClass "/Game/FridayNightFunkin/Blueprints/Arrows/Blueprints/Childs/Standard/BP_Arrow_Standard.BP_Arrow_Standard_C" (Math|Transform|MakeTransform Spawn%20Transform%20Location "0.000000,90.000000,0.000000" "1.000000,1.000000,1.000000") "Undefined" "MultiplyWithRoot" 0 ChanceX Spawn%20Transform%20Location EnumDirection Exemple%20? TimeSpawn TimelineMult Start%20Timer 0))

(event Custom|SpawnHold
  (params (Spawn%20Transform%20Location :type Vector) (HoldDuration :type Float%20%28double-precision%29) (ScaleMult :type Float%20%28double-precision%29) (EnumDirection :type E_Direction%20Enum :default "NewEnumerator0") (TimelineMult :type Float%20%28double-precision%29) (Exemple%20? :type Boolean) (TimeSpawn :type Float%20%28double-precision%29) (Start%20Timer :type Float%20%28double-precision%29))
  ;[0.5 0 0.5 0.5] Spawn Arrow System
  (Game|SpawnActorfromClass "/Game/FridayNightFunkin/Blueprints/Arrows/Blueprints/Childs/Hold/BP_Arrow_Hold.BP_Arrow_Hold_C" (Math|Transform|MakeTransform Spawn%20Transform%20Location "0.000000,90.000000,0.000000" "1.000000,1.000000,1.000000") "Undefined" "MultiplyWithRoot" 0 HoldDuration ScaleMult Spawn%20Transform%20Location EnumDirection Exemple%20? TimeSpawn TimelineMult Start%20Timer 0))

(event Custom|StartLevel
  ;[0.05781 0.117 0.1651] Start The Game
  (CallFunction|Countdown)
  (bind _asbp_controller_f (Utilities|Casting|CastToBP_Controller_F (Game|GetPlayerController 0)))
  (EventDispatchers|BindEventtoEDTest _asbp_controller_f (EventDispatchers|CreateEvent :!event Custom|TimeSet))
  (EventDispatchers|BindEventtoEndGame _asbp_controller_f (EventDispatchers|CreateEvent :!event Custom|TimeSet)))

(event EventBeginPlay
  ;[0.05781 0.117 0.1651] Start The Game
  (Actor|Tick|SetActorTickEnabled false))

(event EventTick
  (params (DeltaSeconds :type Float%20%28single-precision%29))
  (bind _arrowindex (Variables|Spawn|GetArrowIndex))
  (bind _levelpresset (Variables|Game|GetLevelPresset))
  (bind _structure (Variables|/Game/FridayNightFunkin/Levels/BP_LevelPreset.BP_LevelPreset_C|GetStructure _levelpresset))
  (bind _output (Utilities|Array|Get(acopy) _structure _arrowindex))
  ;[1 0 0 0.5] Arrow Patern System
  (Variables|Game|SetCurrentTime (- (Utilities|Time|GetGameTimeinSeconds) (Variables|Game|GetStartTimer)))
  (if (<= (Utilities|Array|Length (Variables|/Game/FridayNightFunkin/Levels/BP_LevelPreset.BP_LevelPreset_C|GetStructure (Variables|Game|GetLevelPresset))) (Variables|Spawn|GetArrowIndex))
    (Actor|Tick|SetActorTickEnabled false)
    (elif (and (not (Utilities|Array|Get(acopy) (Variables|Spawn|GetArrowSpanned?) _arrowindex)) (<= (.starttiming _output) (+ (Variables|Game|GetCurrentTime) (Variables|Spawn|GetArrowTravelTime))))
      (CallFunction|SpawnArrowfromPresset (.starttiming _output) (.holdduration _output) (.tilehold _output) (.exemple? _output) (.direction _output) (.movementduration _output) (.arrowtype _output)))))

(fn ConstructionScript)