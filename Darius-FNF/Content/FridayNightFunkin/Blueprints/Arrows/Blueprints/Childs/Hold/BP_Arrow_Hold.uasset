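; Hold-note arrow for a Friday Night Funkin' rhythm game, requiring sustained input for HoldDuration.
; Construction tints the trail widget by direction and sizes it from ScaleMult.
; ArrowCheck enables Tick, which, while input is held, removes the arrow head, halts movement and plays a duration-scaled Timeline to update and slide the trail.
; Reaching the duration calls ArrowValid; early release stops the Timeline and calls ArrowFail.
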(event EventBeginPlay
  ;[0.05613 0.1144 0.159] BeginPlay
  (|CallParentFunction)
  (Actor|Tick|SetActorTickEnabled false))

(event EventTick
  (params (DeltaSeconds :type Float%20%28single-precision%29))
  (bind _widget (Variables|Default|GetWidget))
  (bind _widget_2 (Variables|Default|GetWidget))
  (bind _as_bp_controller_f_0 (Variables|Default|GetAs%20BP%20Controller%20F_0))
  (bind _relativelocation (Variables|/Script/Engine.SceneComponent|GetRelativeLocation _widget))
  (bind _relativelocation_2 (Variables|/Script/Engine.SceneComponent|GetRelativeLocation _widget_2))
  ;[0.15 1 0.15 0.5] Hold System with tick
  (if (Variables|/Game/FridayNightFunkin/Blueprints/Character/BP_Controller_F.BP_Controller_F_C|GetAction%20Value _as_bp_controller_f_0)
    (if (>= (Variables|/Game/FridayNightFunkin/Blueprints/Character/BP_Controller_F.BP_Controller_F_C|GetTriggered%20Seconds _as_bp_controller_f_0) (Variables|Default|GetHoldDuration))
      (CallFunction|ArrowValid)
      (else
        (Utilities|FlowControl|DoOnce false
          (:Completed
            (Components|DestroyComponent (Variables|Default|GetArrow))
            (Components|Movement|StopMovementImmediately (Variables|Default|GetInterpToMovement))
            (Variables|Default|SetCenter%20Z (/ (* (- (Variables|Default|GetScaleMult) 1.0) 1.5e+02) 2.0))
            (Transformation|SetRelativeLocation _widget_2 (Math|Vector|MakeVector (.x _relativelocation_2) (.y _relativelocation_2) (Variables|Default|GetCenter%20Z)) false true)
            (Components|Timeline|SetPlayRate (Variables|Default|GetTimeline) (/ 1.0 (Variables|Default|GetHoldDuration)))
            (bind _newtrack_0 (Timeline|Timeline PlayFromStart)
              (:Update
                (Default|Update (Variables|Default|GetAs%20WBP%20Hold) _newtrack_0)
                (Transformation|SetRelativeLocation _widget (Math|Vector|MakeVector (.x _relativelocation) (.y _relativelocation) (Math|Float|Lerp (Variables|Default|GetCenter%20Z) (* (+ (Variables|Default|GetCenter%20Z) 75.0) -1.0) _newtrack_0)) false false))
              (:Finished
                (CallFunction|ArrowValid)))))))
    (else
      (Utilities|FlowControl|Sequence
        (:then_0
          (Timeline|Timeline Stop))
        (:then_1
          (CallFunction|ArrowFail))))))

(event EventArrowCheck
  ;[1 0.15 0.15 0.5] Event when the arrow is clicked
  (bind _asbp_controller_f (Utilities|Casting|CastToBP_Controller_F (Game|GetPlayerController 0)))
  (Variables|Default|SetAs%20BP%20Controller%20F_0 _asbp_controller_f)
  (bind _aswbp_hold (Utilities|Casting|CastToWBP_Hold (UserInterface|GetWidget (Variables|Default|GetWidget))))
  (Variables|Default|SetAs%20WBP%20Hold _aswbp_hold)
  (Actor|Tick|SetActorTickEnabled true))

(fn ConstructionScript
  (bind _widget (Variables|Default|GetWidget))
  (bind _widget_2 (Variables|Default|GetWidget))
  (bind _relativelocation (Variables|/Script/Engine.SceneComponent|GetRelativeLocation _widget))
  (bind _relativescale3d (Variables|/Script/Engine.SceneComponent|GetRelativeScale3D _widget_2))
  (switch Utilities|FlowControl|Switch|SwitchonE_Direction (Variables|Default|GetEnumDirection)
    (:NewEnumerator0
      (Variables|Default|SetNew%20Tint%20Color%20and%20Opacity "(R=1.000000,G=0.000000,B=1.000000,A=1.000000)"))
    (:NewEnumerator1
      (Variables|Default|SetNew%20Tint%20Color%20and%20Opacity "(R=0.000000,G=1.000000,B=1.000000,A=1.000000)"))
    (:NewEnumerator2
      (Variables|Default|SetNew%20Tint%20Color%20and%20Opacity "(R=0.000000,G=1.000000,B=0.000000,A=1.000000)"))
    (:NewEnumerator3
      (Variables|Default|SetNew%20Tint%20Color%20and%20Opacity "(R=1.000000,G=0.000000,B=0.000000,A=1.000000)")))
  (Class|WidgetComponent|SetTintColorandOpacity (Variables|Default|GetWidget) (Variables|Default|GetNew%20Tint%20Color%20and%20Opacity))
  (Transformation|SetRelativeScale3D _widget_2 (Math|Vector|MakeVector (.x _relativescale3d) (* (.y _relativescale3d) (- (Variables|Default|GetScaleMult) 1.0)) (.z _relativescale3d)))
  (Transformation|SetRelativeLocation _widget (Math|Vector|MakeVector (.x _relativelocation) (.y _relativelocation) (- (.z _relativelocation) (+ (* (/ (- (Variables|Default|GetScaleMult) 1.0) 2.0) 1.5e+02) 75.0))) false false)
  (|CallParentFunction))