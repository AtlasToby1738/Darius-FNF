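; BP_Arrow_Standard is a standard rhythm-game arrow that can spawn as an X arrow, which loses the game when pressed.
; At construction, arrows flagged CanBeX have a 25% chance to become X and swap their mesh to the MI_X material.
; The press event calls LoseGame on the controller for X arrows and otherwise defers to the parent arrow's logic.
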(event EventArrowGotPressed
  (if (Variables|Default|GetX?)
    (Default|LoseGame (Variables|Default|GetAs%20BP%20Controller%20F))
    (else
      (|CallParentFunction))))

(fn ConstructionScript
  (|CallParentFunction)
  (if (Variables|Default|GetCanBeX?)
    (if (< (Math|Random|RandomFloatinRange 0.0 1e+02) 25.0)
      (Variables|Default|SetX? true)
      (Rendering|Material|SetMaterial (Variables|Default|GetArrow) 0 "/Game/FridayNightFunkin/Materials/Arrows/MI_X.MI_X"))))