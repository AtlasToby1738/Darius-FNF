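; Parent Blueprint for the Friday Night Funkin' note arrows, which travel up to a hit point and get judged on press.
; Construction sets the material by direction and builds the InterpToMovement path, overshooting the hit point unless it is an example arrow.
; Presses are graded in 45 ms steps from the expected arrival time, then reported to BP_Controller_F as score or fail.
; Valid hits spawn a direction-colored, rating-scaled splash; other arrow types route to an empty ArrowCheck hook.
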(event Custom|SpawnSplash
  ;[0.9734 0.5776 0.01681] Spawn the VFX when the arrow is activate
  (bind _returnvalue (Niagara|SpawnSystematLocation "/Game/FridayNightFunkin/Blueprints/Arrows/VFX/ArrowSplash.ArrowSplash" (Variables|VFX|GetVFXSpawnLocation) "0.000000,180.000000,0.000000"))
  (bind _output_get (Variables|VFX|SetVFX _returnvalue))
  (Niagara|SetNiagaraVariable(Float) _output_get "AmountParticul" (Utilities|Select :Index (Variables|Type|GetHitType) :NewEnumerator0 2e+02 :NewEnumerator1 1e+02 :NewEnumerator2 5e+01 :NewEnumerator3 1e+01 :NewEnumerator4 0.0 :NewEnumerator5 0.0))
  (Niagara|SetNiagaraVariable(LinearColor) (Variables|VFX|GetVFX) "NewColor" (Utilities|Array|Get(acopy) (Variables|VFX|GetColorArray) (Utilities|Select :Index (Variables|Type|GetEnumDirection) :NewEnumerator0 0 :NewEnumerator1 1 :NewEnumerator2 2 :NewEnumerator3 3))))

(event Custom|ArrowValid
  (bind _index (Variables|Score|GetIndex))
  (bind _tablescore (Variables|Score|GetTableScore))
  (bind _output (Utilities|Array|Get(acopy) _tablescore _index))
  ;[0.1095 0.1845 0.0999] Valid the score
  (Variables|Type|SetHitType (Utilities|Select :Index (Variables|Score|GetIndex) :Option%200 "NewEnumerator0" :Option%201 "NewEnumerator1" :Option%202 "NewEnumerator2" :Option%203 "NewEnumerator3"))
  (bind _output_get (Variables|Score|SetScore (Utilities|Select :Index (Variables|Type|GetHitType) :NewEnumerator0 _output :NewEnumerator1 _output :NewEnumerator2 _output :NewEnumerator3 _output :NewEnumerator4 0.0 :NewEnumerator5 0.0)))
  (Default|Score (Variables|refs|GetAs%20BP%20Controller%20F) _output_get _index)
  (CallFunction|SpawnSplash)
  (Actor|DestroyActor))

(event Custom|ArrowCheck
  ;[0.1195 0.1221 0.1195] When the Arrow is pressed, we check if the arrow is in the range to get scored
)

(event Custom|ArrowFail
  ;[1 0.03955 0.03955] Fail And Miss
  (Variables|Type|SetHitType "NewEnumerator5")
  (Default|Fail (Variables|refs|GetAs%20BP%20Controller%20F))
  (Actor|DestroyActor))

(event Custom|ArrowMiss
  ;[1 0.03955 0.03955] Fail And Miss
  (Variables|Type|SetHitType "NewEnumerator4")
  (Actor|DestroyActor))

(event Custom|ArrowGotPressed
  (bind _returnvalue (Utilities|Time|GetGameTimeinSeconds))
  (bind _timespawn (Variables|Movement|GetTimeSpawn))
  (bind _movementduration (Variables|Movement|GetMovementDuration))
  (bind _arrow (Variables|Default|GetArrow))
  (bind _start_timer (Variables|Movement|GetStart%20Timer))
  (bind _returnvalue_2 (+ _timespawn _movementduration))
  (bind _returnvalue_3 (- _returnvalue _start_timer))
  (bind _returnvalue_4 (- _returnvalue_2 _returnvalue_3))
  (bind _returnvalue_5 (/ _returnvalue_4 0.045))
  ;[0.1195 0.1221 0.1195] When the Arrow is pressed, we check if the arrow is in the range to get scored
  (Utilities|IsValid _arrow
    (:Is%20Valid
      (Variables|VFX|SetVFXSpawnLocation (Transformation|GetWorldLocation _arrow)))
    (:Is%20Not%20Valid
      _))
  (Variables|Score|SetIndex (Math|Integer|Absolute(Integer) (Math|Float|Truncate _returnvalue_5)))
  (if (and (>= _returnvalue_5 -4.0) (<= _returnvalue_5 4.0))
    (if (Utilities|Enum|Equal(Enum) "NewEnumerator0" (Variables|Type|GetArrowsType))
      (CallFunction|ArrowValid)
      (else
        (CallFunction|ArrowCheck)))
    (else
      (CallFunction|ArrowFail))))

(event EventBeginPlay
  ;[0 0.3864 0.8796] BeginPlay
  (bind _asbp_controller_f (Utilities|Casting|CastToBP_Controller_F (Game|GetPlayerController 0)))
  (Variables|refs|SetAs%20BP%20Controller%20F _asbp_controller_f)
  (if (Variables|Type|GetExemple%20?)
    (Utilities|FlowControl|Delay (Variables|Movement|GetMovementDuration))
    (Actor|DestroyActor)))

(fn ConstructionScript
  (bind _startpoint (Variables|Movement|GetStartPoint))
  (bind _arrow (Variables|Default|GetArrow))
  (Class|InterptoMovementComponent|AddControlPointPosition (Variables|Default|GetInterpToMovement) (Variables|Movement|GetStartPoint) false)
  (bind _output_get (Variables|Movement|SetHitPoint (Math|Vector|MakeVector (.x _startpoint) (.y _startpoint) (+ (.z _startpoint) 8e+02))))
  (Class|InterptoMovementComponent|AddControlPointPosition (Variables|Default|GetInterpToMovement) _output_get false)
  (if (Variables|Type|GetExemple%20?)
    (Variables|/Script/Engine.InterpToMovementComponent|SetDuration (Variables|Default|GetInterpToMovement) (Variables|Movement|GetMovementDuration))
    (else
      (Class|InterptoMovementComponent|AddControlPointPosition (Variables|Default|GetInterpToMovement) (Math|Vector|MakeVector (.x (Variables|Movement|GetHitPoint)) (.y (Variables|Movement|GetHitPoint)) (+ (.z (Variables|Movement|GetHitPoint)) 2e+02)) false)
      (Variables|/Script/Engine.InterpToMovementComponent|SetDuration (Variables|Default|GetInterpToMovement) (* (Variables|Movement|GetMovementDuration) 1.25))))
  (switch Utilities|FlowControl|Switch|SwitchonE_Direction (Variables|Type|GetEnumDirection)
    (:NewEnumerator0
      (Rendering|Material|SetMaterial _arrow 0 "/Game/FridayNightFunkin/Materials/Arrows/MM_Left_Arrow.MM_Left_Arrow"))
    (:NewEnumerator1
      (Rendering|Material|SetMaterial _arrow 0 "/Game/FridayNightFunkin/Materials/Arrows/MI_Down_Arrow.MI_Down_Arrow"))
    (:NewEnumerator2
      (Rendering|Material|SetMaterial _arrow 0 "/Game/FridayNightFunkin/Materials/Arrows/MI_Up_Arrow.MI_Up_Arrow"))
    (:NewEnumerator3
      (Rendering|Material|SetMaterial _arrow 0 "/Game/FridayNightFunkin/Materials/Arrows/MI_Right_Arrow.MI_Right_Arrow"))))