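; BP_DeadZone is a trigger box that catches arrows in a Friday Night Funkin-style rhythm game and registers misses.
; On BeginPlay it caches the player's BP_Controller_F.
; When an actor overlaps the box, it calls Fail on that controller, unless the actor is a BP_Arrow_Standard with its X flag set.
; The overlapping actor is then destroyed, so flagged standard arrows are removed without a fail.
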(event OnComponentBeginOverlap(Box)
  (params (OverlappedComponent :type Primitive%20Component%20Object%20Reference) (OtherActor :type Actor%20Object%20Reference) (OtherComp :type Primitive%20Component%20Object%20Reference) (OtherBodyIndex :type Integer) (bFromSweep :type Boolean) (SweepResult :type Hit%20Result%20Structure%20%28by%20ref%29))
  ;[0.15 0.02734 0.02734 0.5] Fail arrow when it hit the box
  (bind _output_get (Variables|Default|SetOther%20Actor OtherActor))
  (if (== (Utilities|GetClass _output_get) "/Game/FridayNightFunkin/Blueprints/Arrows/Blueprints/Childs/Standard/BP_Arrow_Standard.BP_Arrow_Standard_C")
    (bind _asbp_arrow_standard (Utilities|Casting|CastToBP_Arrow_Standard (Variables|Default|GetOther%20Actor)))
    (if (Variables|/Game/FridayNightFunkin/Blueprints/Arrows/Blueprints/Childs/Standard/BP_Arrow_Standard.BP_Arrow_Standard_C|GetX? _asbp_arrow_standard)
      _
      (else
        (Default|Fail (Variables|Default|GetAs%20BP%20Controller%20F) :!label _label)))
    (else
      (goto _label)))
  (Actor|DestroyActor (Variables|Default|GetOther%20Actor)))

(event EventBeginPlay
  (bind _asbp_controller_f (Utilities|Casting|CastToBP_Controller_F (Game|GetPlayerController 0)))
  (Variables|Default|SetAs%20BP%20Controller%20F _asbp_controller_f))

(event Collision|EventActorBeginOverlap
  (params (OtherActor :type Actor%20Object%20Reference)))

(event EventTick
  (params (DeltaSeconds :type Float%20%28single-precision%29)))

(fn ConstructionScript)